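; Shao Kahn boss character that sets its name, health, death montage and boss health bar widget at start.
; Point damage reduces health in the enemy component, doubles on head hits and is reported as a damage event, with death removing the bar.
; Equipping shows the bar and plays a montage whose notify spawns the staff weapon on a socket.
; Unequipping hides the bar and destroys the weapon on its montage notify.
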(event `self.ReceiveTick`
  (params (DeltaSeconds :type "Float (single-precision)"))
  (`parent.ReceiveTick` DeltaSeconds))

(event `self.ReceiveBeginPlay`
  (bind _bpc_enemy (`self.BPC_Enemy`))
  (`parent.ReceiveBeginPlay`)
  (set `/Game/AI_Tests_Tests/BossAnimationsPack/AI_Characters/AI_Enemy_Base/BPC_Enemy.EnemyName` "Младший сын" (`self.BPC_Enemy`))
  (set `self.DeathMontage` "/Game/AI_Tests_Tests/BossAnimationsPack/AI_Characters/AI_Shao_Kahn/Animations/Death/BossDeathLong_Montage.BossDeathLong_Montage")
  (bind _output_get (set `/Game/AI_Tests_Tests/BossAnimationsPack/AI_Characters/AI_Enemy_Base/BPC_Enemy.MaxHealth` (`self.BossHealth`) _bpc_enemy))
  (set `/Game/AI_Tests_Tests/BossAnimationsPack/AI_Characters/AI_Enemy_Base/BPC_Enemy.Health` _output_get _bpc_enemy)
  (bind _returnvalue (`|CreateWidget` "/Game/AI_Tests_Tests/BossAnimationsPack/AI_Characters/AI_Enemy_Base/Bar_for_Boss/BossWitoutArmor/W_HealthBar_Boss.W_HealthBar_Boss_C" null self))
  (set `self.BossBar` _returnvalue)
  (add `self.OnTakePointDamage` (delegate `OnTakePointDamage_Event`)))

(event `OnTakePointDamage_Event`
  (params (DamagedActor :type "Actor Object Reference") (Damage :type "Float (single-precision)") (InstigatedBy :type "Controller Object Reference") (HitLocation :type "Vector Structure") (FHitComponent :type "PrimitiveComponent Object Reference") (BoneName :type Name) (ShotFromDirection :type "Vector Structure") (DamageType :type "DamageType Object Reference") (DamageCauser :type "Actor Object Reference"))
  (bind _bpc_enemy (`self.BPC_Enemy`))
  ;[1 0.05098 0] Apply Damage And Death via c++
  (set `self.Hit Location` HitLocation)
  (bind _output_get (set `/Game/AI_Tests_Tests/BossAnimationsPack/AI_Characters/AI_Enemy_Base/BPC_Enemy.Health` (- (`/Game/AI_Tests_Tests/BossAnimationsPack/AI_Characters/AI_Enemy_Base/BPC_Enemy.Health` _bpc_enemy) (* Damage (`KismetMathLibrary.SelectFloat` 2.0 1.0 (== BoneName "head")))) _bpc_enemy))
  (`AISense_Damage.ReportDamageEvent` DamagedActor InstigatedBy Damage ShotFromDirection)
  (if (<= _output_get 0.0)
    (`/Engine/EditorBlueprintResources/StandardMacros.DoOnce` false
      (:`Completed`
        (`self.DiedEnemy`)))))

(event `DiedEnemy`
  ;[1 1 1] Died
  (bind _bossbar (`self.BossBar`)
    (:`then`
      (`Widget.RemoveFromParent` _bossbar))
    (:`else`
      _))
  (`self.AI_Death` null))

(event `/Game/AI_Tests_Tests/BossAnimationsPack/AI_Characters/AI_Enemy_Base/BPI_Enemy.EquipWeapon`
  ;[1 1 1] Equip Weapon
  (`UserWidget.AddToViewport` (`self.BossBar`) 0)
  (set `self.AttackState` true)
  (set `self.IsWeildingWeapon` true)
  (bind _notifyname (`|PlayMontage` (`self.Mesh`) "/Game/AI_Tests_Tests/BossAnimationsPack/AI_Characters/AI_Berserk/Animation_Berserk/Sword_Anim_Pack/01_Idle/Idle_To_Combat.Idle_To_Combat")
    (:`OnCompleted`
      (`self.OnWealdAxe`))
    (:`OnNotifyBegin`
      (switch `name` _notifyname
        (:`HoldAxe`
          (bind _returnvalue (`|SpawnActorFromClass` "/Game/AI_Tests_Tests/BossAnimationsPack/AI_Characters/Weapon_AI/Shao_Kahn/BB_Weapon_Shao_Kahn.BB_Weapon_Shao_Kahn_C" (`self.GetTransform`) "Undefined" "MultiplyWithRoot" null null))
          (bind _output_get (set `self.WeaponActor` _returnvalue))
          (`self.K2_AttachToComponent` _output_get (`self.Mesh`) "Staff" "SnapToTarget" "SnapToTarget" "SnapToTarget" true))))))

(event `/Game/AI_Tests_Tests/BossAnimationsPack/AI_Characters/AI_Enemy_Base/BPI_Enemy.UnequipWeapon`
  (bind _bossbar (`self.BossBar`))
  ;[1 1 1] Unequip Weapon
  (`/Engine/EditorBlueprintResources/StandardMacros.IsValid` _bossbar
    (:`Is Valid`
      (`Widget.RemoveFromParent` _bossbar)
      (set `self.AttackState` false)
      (bind _notifyname (`|PlayMontage` (`self.Mesh`) "/Game/AI_Tests_Tests/BossAnimationsPack/AI_Characters/AI_Berserk/Animation_Berserk/Sword_Anim_Pack/01_Idle/Combat_To_Idle.Combat_To_Idle")
        (:`then`
          (`self.OnSheathAxe`))
        (:`OnNotifyBegin`
          (switch `name` _notifyname
            (:`DropAxe`
              (`self.K2_DestroyActor` (`self.WeaponActor`))
              (set `self.IsWeildingWeapon` false))))))))

(fn `Get CurrentHealth`
  (returns (Health :type "Float (double-precision)"))
  (return (`/Game/AI_Tests_Tests/BossAnimationsPack/AI_Characters/AI_Enemy_Base/BPC_Enemy.Health` (`self.BPC_Enemy`))))

(fn `Get MaxHealth`
  (returns (MaxHealth :type "Float (double-precision)"))
  (return (`/Game/AI_Tests_Tests/BossAnimationsPack/AI_Characters/AI_Enemy_Base/BPC_Enemy.MaxHealth` (`self.BPC_Enemy`))))

(fn `GetEnemyName`
  (returns (Name :type Text))
  (return (`/Game/AI_Tests_Tests/BossAnimationsPack/AI_Characters/AI_Enemy_Base/BPC_Enemy.EnemyName` (`self.BPC_Enemy`))))

(fn `UserConstructionScript`
  (`parent.UserConstructionScript`))