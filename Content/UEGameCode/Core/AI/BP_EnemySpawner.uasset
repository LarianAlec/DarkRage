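; BP_EnemySpawner is a placed actor that keeps spawning BP_AI_Enemy pawns at its billboard's location on a looping timer.
; Each pawn is spawned with BT_Enemy, takes the spawner's configured AI state, and has that state written to its blackboard.
; The spawner then gives it a random speed capped at its chase speed and flags it as already warned.
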(event `self.ReceiveBeginPlay`
  (`KismetSystemLibrary.K2_SetTimerDelegate` (delegate `SpawnEnemy`) (`self.SpanRate`) true))

(event `SpawnEnemy`
  (bind _billboard (`self.Billboard`))
  (bind _pawn (`self.Pawn`))
  (bind _returnvalue (`AIBlueprintHelperLibrary.SpawnAIFromClass` "/Game/UEGameCode/Core/AI/BP_AI_Enemy.BP_AI_Enemy_C" "/Game/UEGameCode/Core/AI/BT_Enemy.BT_Enemy" (`SceneComponent.K2_GetComponentLocation` _billboard) (`SceneComponent.K2_GetComponentRotation` _billboard) false null))
  (bind _asbp_ai_enemy (cast `/Game/UEGameCode/Core/AI/BP_AI_Enemy` _returnvalue))
  (bind _output_get (set `self.Pawn` _asbp_ai_enemy))
  (bind _output_get_2 (set `/Game/UEGameCode/Core/AI/BP_AI_Enemy.PatrolState` (`self.AIState`) _output_get))
  (`BlackboardComponent.SetValueAsEnum` (`AIBlueprintHelperLibrary.GetBlackboard` (`AIBlueprintHelperLibrary.GetAIController` (`self.Pawn`))) "AIState" _output_get_2)
  (`/Game/UEGameCode/Core/AI/BP_AI_Enemy.UpdateSpeed` _pawn (`KismetMathLibrary.RandomFloatInRange` 300.0 (`/Game/UEGameCode/Core/AI/BP_AI_Enemy.ChaseSpeed` _pawn)))
  (set `/Game/UEGameCode/Core/AI/BP_AI_Enemy.IsWarned` true (`self.Pawn`)))

(fn `UserConstructionScript`)