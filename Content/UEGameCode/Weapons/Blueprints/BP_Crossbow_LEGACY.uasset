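; Legacy crossbow weapon that fires hitscan shots and plays first-person fire and reload montages on the player's arms mesh.
; Fire is gated by reload and firing flags, traces as the montage starts, sends damage through BPI_Damage, and resets after a shot delay.
; Reload clears its flag on montage blend-out, or after a delay if interrupted; CancelReload stops the montage immediately.
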(event `self.ReceiveBeginPlay`
  (`parent.ReceiveBeginPlay`)
  (set `self.Damage` (`self.CrossbowRegularDamage`)))

(event `self.Fire`
  ;[1 1 1] Firing
  (if (not (`self.IsReloading`))
    (if (not (`self.IsFiring`))
      ;;[1 1 1] Play Animation
      (set `self.IsFiring` true)
      (`|PlayMontage` (`/Game/UEGameCode/Core/Blueprints/BP_DarkRageCharacter_LEGACY.Mesh1P` (`self.PlayerRef`)) "/Game/UEGameCode/Characters/1P_TemplateManequin/Animations/AssetAnimations/FP_Fire_Montage.FP_Fire_Montage"
        (:`then`
          ;;[1 1 1] Fire Hitscan
          (bind _hitinfol (`self.Fire_Hitscan` true))
          (`|ExecutionSequence`
            (:`then_0`
              (`GameplayStatics.SpawnSoundAttached` "/Game/DarkRage/Core/Weapons/Crossbow/Audio/CrossbowShoot_Cue.CrossbowShoot_Cue" (`self.DefaultSceneRoot`) "None" (0.0 0.0 0.0) (struct) "KeepRelativeOffset" false 1.0 1.0 0.0 null null)
              (`KismetSystemLibrary.Delay` (`self.DelayBetweenShoots`))
              (set `self.IsFiring` false))
            (:`then_1`
              (bind (_bblockinghit _binitialoverlap _time _distance _location _impactpoint _normal _impactnormal _physmat _hitactor _hitcomponent _hitbonename) (`GameplayStatics.BreakHitResult` _hitinfol))
              ;[1 1 1] Applying Damage
              (if (`KismetSystemLibrary.DoesImplementInterface` _hitactor "/Game/UEGameCode/Core/Interfaces/BPI_Damage.BPI_Damage_C")
                (message `/Game/UEGameCode/Core/Interfaces/BPI_Damage.ReceiveDamage` _hitactor (`self.Damage`) _impactpoint _hitbonename)))))))))

(event `self.Reload`
  ;[1 1 1] Reloading
  (if (not (`self.IsReloading`))
    (set `self.IsReloading` true)
    (`|PlayMontage` (`/Game/UEGameCode/Core/Blueprints/BP_DarkRageCharacter_LEGACY.Mesh1P` (`self.PlayerRef`)) "/Game/UEGameCode/Characters/1P_TemplateManequin/Animations/AssetAnimations/FP_Reload_Montage.FP_Reload_Montage"
      (:`OnBlendOut`
        _)
      (:`OnInterrupted`
        (`KismetSystemLibrary.Delay` 1.0)))
    (set `self.IsReloading` false)))

(event `self.CancelReload`
  ;[1 1 1] Cancel Reload
  (`AnimInstance.Montage_Stop` (`SkeletalMeshComponent.GetAnimInstance` (`/Game/UEGameCode/Core/Blueprints/BP_DarkRageCharacter_LEGACY.Mesh1P` (`self.PlayerRef`))) 0.0 null))

(fn `UserConstructionScript`
  (`parent.UserConstructionScript`))