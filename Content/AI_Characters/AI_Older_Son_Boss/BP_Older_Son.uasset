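; Older Son boss character that fights with spear and shield, with a boss bar created for its health and armor.
; Point damage, doubled on headshots, drains armor before health; breaking armor stows the shield, and zero health triggers death.
; A second-stage event restores armor and re-equips the shield, with montage notifies destroying and respawning gear on hand or idle sockets.
; A timeline lerps dash attacks, and a landed delegate stops jump-attack movement.
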(event `self.ReceiveBeginPlay`
  (bind _bpc_enemy (`self.BPC_Enemy`))
  (bind _pawnhealth (`self.PawnHealth`))
  (bind _pawnarmor (`self.PawnArmor`))
  (`parent.ReceiveBeginPlay`)
  (set `/Game/AI_Characters/AI_Enemy_Base/BPC_Enemy.BurstBerserk` true (`self.BPC_Enemy`))
  (bind _returnvalue (`|SpawnActorFromClass` "/Game/AI_Characters/Weapon_AI/Bear_Boss/BP_Bear_Spear.BP_Bear_Spear_C" (`self.GetTransform`) "Undefined" "MultiplyWithRoot" null null))
  (bind _output_get (set `self.WeaponActor` _returnvalue))
  (`self.K2_AttachToComponent` _output_get (`self.Mesh`) "SpearIdle" "SnapToTarget" "SnapToTarget" "SnapToTarget" true)
  (bind _returnvalue_2 (`|SpawnActorFromClass` "/Game/AI_Characters/Weapon_AI/OlderSon/BP_ShieldBoss.BP_ShieldBoss_C" (`self.GetTransform`) "Undefined" "MultiplyWithRoot" null null))
  (bind _output_get_2 (set `self.ShieldActor` _returnvalue_2))
  (`self.K2_AttachToComponent` _output_get_2 (`self.Mesh`) "ShieldIdle" "SnapToTarget" "SnapToTarget" "SnapToTarget" true)
  (set `/Game/AI_Characters/AI_Enemy_Base/BPC_Enemy.EnemyName` "Старший сын" (`self.BPC_Enemy`))
  (set `self.DeathMontage` "/Game/AI_Characters/AI_Bear_Boss/Animation/Frank_RPG_Spear/Animations/Mannequin/Frank_RPG_Spear_Die05_Montage.Frank_RPG_Spear_Die05_Montage")
  (set `/Game/AI_Characters/AI_Enemy_Base/BPC_Enemy.Health` _pawnhealth _bpc_enemy)
  (set `/Game/AI_Characters/AI_Enemy_Base/BPC_Enemy.MaxHealth` _pawnhealth _bpc_enemy)
  (set `/Game/AI_Characters/AI_Enemy_Base/BPC_Enemy.Armor` _pawnarmor _bpc_enemy)
  (set `/Game/AI_Characters/AI_Enemy_Base/BPC_Enemy.MaxArmor` _pawnarmor _bpc_enemy)
  (bind _returnvalue_3 (`|CreateWidget` "/Game/AI_Characters/AI_Enemy_Base/Bar_for_Boss/BossWithArmo/W_HealthBarAI_testArmor.W_HealthBarAI_testArmor_C" null self))
  (set `self.BossBar` _returnvalue_3)
  (add `self.OnTakePointDamage` (delegate `OnTakePointDamage_Event`)))

(event `OnTakePointDamage_Event`
  (params (DamagedActor :type "Actor Object Reference") (Damage :type "Float (single-precision)") (InstigatedBy :type "Controller Object Reference") (HitLocation :type "Vector Structure") (FHitComponent :type "PrimitiveComponent Object Reference") (BoneName :type Name) (ShotFromDirection :type "Vector Structure") (DamageType :type "DamageType Object Reference") (DamageCauser :type "Actor Object Reference"))
  (bind _bpc_enemy (`self.BPC_Enemy`))
  (bind _bpc_enemy_2 (`self.BPC_Enemy`))
  (bind _health (`/Game/AI_Characters/AI_Enemy_Base/BPC_Enemy.Health` _bpc_enemy_2))
  (bind _armor (`/Game/AI_Characters/AI_Enemy_Base/BPC_Enemy.Armor` _bpc_enemy_2))
  ;[1 1 1] TakeDamage
  (`NiagaraFunctionLibrary.SpawnSystemAtLocation` "/Game/VFX/P_Splash_SkMesh_Stylized.P_Splash_SkMesh_Stylized" HitLocation (struct) (0.3 0.3 0.3))
  (`AISense_Damage.ReportDamageEvent` DamagedActor InstigatedBy 0.0 HitLocation)
  (set `self.Hit Location` HitLocation)
  (set `self.ReciveDamage` (* (`self.HealthMult`) (* Damage (`KismetMathLibrary.SelectFloat` 2.0 1.0 (== BoneName "head")))))
  (if (== _armor 0.0)
    (bind _output_get (set `/Game/AI_Characters/AI_Enemy_Base/BPC_Enemy.Health` (- _health (`self.ReciveDamage`)) (`self.BPC_Enemy`)))
    (if (<= _output_get 0.0)
      (`self.Death`))
    (elif (> (`self.ReciveDamage`) _armor)
      (`self.UnpinShield`)
      (bind _output_get_2 (set `/Game/AI_Characters/AI_Enemy_Base/BPC_Enemy.Health` (- (+ _armor _health) (`self.ReciveDamage`)) _bpc_enemy))
      (set `/Game/AI_Characters/AI_Enemy_Base/BPC_Enemy.Armor` 0.0 _bpc_enemy)
      (if (<= _output_get_2 0.0)
        (`self.Death`))
      (else
        (bind _output_get_3 (set `/Game/AI_Characters/AI_Enemy_Base/BPC_Enemy.Armor` (- _armor (`self.ReciveDamage`)) (`self.BPC_Enemy`)))
        (if (<= _output_get_3 0.0)
          (`self.StopAnimMontage` null)
          (`self.UnpinShield`))))))

(event `Death`
  ;[1 1 1] Death
  (bind _bossbar (`self.BossBar`)
    (:`then`
      (`Widget.RemoveFromParent` _bossbar))
    (:`else`
      _))
  (bind _shieldactor (`self.ShieldActor`)
    (:`then`
      (`self.AI_Death` _shieldactor))
    (:`else`
      (`self.AI_Death` null))))

(event `/Game/AI_Characters/AI_Enemy_Base/BPI_Enemy.EquipWeapon`
  ;[1 1 1] Equip Both
  (`UserWidget.AddToPlayerScreen` (`self.BossBar`) 0)
  (bind _notifyname (`|PlayMontage` (`self.Mesh`) "/Game/AI_Characters/AI_Older_Son_Boss/Animation/UsedSSA/equip_unequip/equip_Montage.equip_Montage")
    (:`OnCompleted`
      (`self.OnWealdAxe`))
    (:`OnNotifyBegin`
      (switch `name` _notifyname
        (:`Hold`
          (bind _shieldactor (`self.ShieldActor`)
            (:`then`
              (`self.K2_DestroyActor` _shieldactor))
            (:`else`
              _))
          (bind _weaponactor (`self.WeaponActor`)
            (:`then`
              (`self.K2_DestroyActor` _weaponactor))
            (:`else`
              _))
          (bind _returnvalue (`|SpawnActorFromClass` "/Game/AI_Characters/Weapon_AI/Bear_Boss/BP_Bear_Spear.BP_Bear_Spear_C" (`self.GetTransform`) "Undefined" "MultiplyWithRoot" null null))
          (bind _output_get (set `self.WeaponActor` _returnvalue))
          (`self.K2_AttachToComponent` _output_get (`self.Mesh`) "hand_rSocket" "SnapToTarget" "SnapToTarget" "SnapToTarget" true)
          (bind _returnvalue_2 (`|SpawnActorFromClass` "/Game/AI_Characters/Weapon_AI/OlderSon/BP_ShieldBoss.BP_ShieldBoss_C" (`self.GetTransform`) "Undefined" "MultiplyWithRoot" null null))
          (bind _output_get_2 (set `self.ShieldActor` _returnvalue_2))
          (`self.K2_AttachToComponent` _output_get_2 (`self.Mesh`) "hand_lSocket" "SnapToTarget" "SnapToTarget" "SnapToTarget" true)
          (set `self.IsWeildingWeapon` true))))))

(event `/Game/AI_Characters/AI_Enemy_Base/BPI_Enemy.EquipWeaponBossStage Second`
  ;[1 1 1] Equip Shield
  (set `/Game/AI_Characters/AI_Enemy_Base/BPC_Enemy.BurstBerserk` false (`self.BPC_Enemy`))
  (set `/Game/AI_Characters/AI_Enemy_Base/BPC_Enemy.Armor` (`self.PawnArmor`) (`self.BPC_Enemy`))
  (bind _notifyname (`|PlayMontage` (`self.Mesh`) "/Game/AI_Characters/AI_Older_Son_Boss/Animation/UsedESSA/EquipShield/Equip_04_Seq_Montage.Equip_04_Seq_Montage" 0.75)
    (:`OnCompleted`
      (`self.OnWealdShield`))
    (:`OnNotifyBegin`
      (switch `name` _notifyname
        (:`Hold`
          (bind _shieldactor (`self.ShieldActor`)
            (:`then`
              (`self.K2_DestroyActor` _shieldactor))
            (:`else`
              _))
          (bind _returnvalue (`|SpawnActorFromClass` "/Game/AI_Characters/Weapon_AI/OlderSon/BP_ShieldBoss.BP_ShieldBoss_C" (`self.GetTransform`) "Undefined" "MultiplyWithRoot" null null))
          (bind _output_get (set `self.ShieldActor` _returnvalue))
          (`self.K2_AttachToComponent` _output_get (`self.Mesh`) "hand_lSocket" "SnapToTarget" "SnapToTarget" "SnapToTarget" true)
          (set `self.IsWeildingWeapon` true)
          (set `self.OnlySpearWeapon` false))))))

(event `UnpinShield`
  ;[1 1 1] UnpinShield
  (bind _notifyname (`|PlayMontage` (`self.Mesh`) "/Game/AI_Characters/AI_Older_Son_Boss/Animation/UsedSSA/Defence_breaked_Montage.Defence_breaked_Montage")
    (:`OnCompleted`
      (set `self.OnlySpearWeapon` true)
      (set `self.IsWeildingWeapon` false))
    (:`OnNotifyBegin`
      (switch `name` _notifyname
        (:`ShieldIdle`
          (bind _shieldactor (`self.ShieldActor`)
            (:`then`
              (`self.K2_DestroyActor` _shieldactor))
            (:`else`
              _))
          (bind _returnvalue (`|SpawnActorFromClass` "/Game/AI_Characters/Weapon_AI/OlderSon/BP_ShieldBoss.BP_ShieldBoss_C" (`self.GetTransform`) "Undefined" "MultiplyWithRoot" null null))
          (bind _output_get (set `self.ShieldActor` _returnvalue))
          (`self.K2_AttachToComponent` _output_get (`self.Mesh`) "ShieldIdle" "SnapToTarget" "SnapToTarget" "SnapToTarget" true))))))

(event `DashTimeLine`
  ;[1 1 1] DashAttackLine
  (set `self.StartLocation` (`self.K2_GetActorLocation`))
  (bind (_direction _longattack) (`Timeline|Timeline` :!via `PlayFromStart`)
    (:`Update`
      (`self.K2_SetActorLocation` (`KismetMathLibrary.VLerp` (`self.StartLocation`) (`self.EndLocation`) _longattack)))))

(event `for jump attack`
  ;[1 1 1] ForJump
  (add `self.LandedDelegate` (delegate `LandedDelegate_Event`)))

(event `LandedDelegate_Event` :!signature `self.LandedDelegate`
  (params (Hit :type "HitResult Structure (by ref)"))
  ;[1 1 1] ForJump
  (remove `self.LandedDelegate` (delegate `LandedDelegate_Event`))
  (`MovementComponent.StopMovementImmediately` (`self.CharacterMovement`)))

(fn `Get CurrentArmor`
  (returns (CurrentArmor :type "Float (double-precision)"))
  (return (`/Game/AI_Characters/AI_Enemy_Base/BPC_Enemy.Armor` (`self.BPC_Enemy`))))

(fn `Get CurrentHealth`
  (returns (Health :type "Float (double-precision)"))
  (return (`/Game/AI_Characters/AI_Enemy_Base/BPC_Enemy.Health` (`self.BPC_Enemy`))))

(fn `Get MaxArmor`
  (returns (MaxArmor :type "Float (double-precision)"))
  (return (`/Game/AI_Characters/AI_Enemy_Base/BPC_Enemy.MaxArmor` (`self.BPC_Enemy`))))

(fn `Get MaxHealth`
  (returns (MaxHealth :type "Float (double-precision)"))
  (return (`/Game/AI_Characters/AI_Enemy_Base/BPC_Enemy.MaxHealth` (`self.BPC_Enemy`))))

(fn `GetEnemyName`
  (returns (Name :type Text))
  (return (`/Game/AI_Characters/AI_Enemy_Base/BPC_Enemy.EnemyName` (`self.BPC_Enemy`))))

(fn `UserConstructionScript`
  (`parent.UserConstructionScript`))