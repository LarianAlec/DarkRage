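; Boss character Blueprint that turns to face the player until death and exposes a damage-window flag.
; AnyDamage, rate-limited by a DoOnce, reduces health, shakes the camera and starts a physics hit reaction.
; A timeline drives the bone physics blend weight, applied each tick with a physical animation profile while alive.
; At zero health it stops AI logic and sets Death on the Shao Kahn anim instance.
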(event `DoDamage`
  ;[1 1 1] Do/Don't damage
  (set `self.Is_Damage_Time` true))

(event `DontDamage`
  ;[1 1 1] Do/Don't damage
  (set `self.Is_Damage_Time` false))

(event `self.ReceiveTick`
  (params (DeltaSeconds :type "Float (single-precision)"))
  (bind (_returnvalue_roll _returnvalue_pitch _returnvalue_yaw) (`KismetMathLibrary.BreakRotator` (`KismetMathLibrary.FindLookAtRotation` (`self.K2_GetActorLocation`) (`self.K2_GetActorLocation` (`GameplayStatics.GetPlayerPawn` 0)))))
  ;[1 1 1] Turn characters face to the player
  (if (not (`self.Death`))
    (`self.K2_SetActorRotation` (`KismetMathLibrary.MakeRotator` 0.0 0.0 (- _returnvalue_yaw 5.0)))
    (`self.PhysicalHitReact`)))

(event `self.ReceiveAnyDamage`
  (params (Damage :type "Float (single-precision)") (DamageType :type "DamageType Object Reference") (InstigatedBy :type "Controller Object Reference") (DamageCauser :type "Actor Object Reference"))
  ;[1 1 1] Get damage
  (`/Engine/EditorBlueprintResources/StandardMacros.DoOnce` false :!label _label
    (:`Completed`
      (`|ExecutionSequence`
        (:`then_0`
          (set `self.current_health` (- (`self.current_health`) Damage))
          (if (<= (`self.current_health`) 0.0)
            ;[1 1 1] Death
            (bind _asabai_shao_kahn (cast `/Game/AI_Tests_Tests/BossAnimationsPack/AI/AI_Shao_Kahn/ABAI_Shao_Kahn` (`SkeletalMeshComponent.GetAnimInstance` (`self.Mesh`))))
            (`BrainComponent.StopLogic` (`AIController.BrainComponent` (`AIBlueprintHelperLibrary.GetAIController` self)) "")
            (set `/Game/AI_Tests_Tests/BossAnimationsPack/AI/AI_Shao_Kahn/ABAI_Shao_Kahn.Death` true _asabai_shao_kahn)
            (set `self.Death` true)
            (else
              (`KismetSystemLibrary.Delay` 0.3)
              (goto _label :!via `Reset`))))
        (:`then_1`
          (`SkeletalMeshComponent.SetAllBodiesBelowSimulatePhysics` (`self.Mesh`) (`self.BoneName`) true true)
          (bind (_direction _newtrack_0) (`Timeline|PhysicsTimeline` :!via `PlayFromStart`)
            (:`Update`
              (set `self.Physics Blend Weight` _newtrack_0)
              (`PrimitiveComponent.AddImpulse` (`self.Mesh`) (200.0 200.0 0.0) "spine_01" false))
            (:`Finished`
              (`SkeletalMeshComponent.SetAllBodiesBelowSimulatePhysics` (`self.Mesh`) (`self.BoneName`) false true))))
        (:`then_2`
          ;[1 1 1] Screen shake
          (`Timeline|ScreenShakeTimeline` :!via `PlayFromStart`
            (:`Update`
              (`GameplayStatics.PlayWorldCameraShake` "/Game/AI_Tests_Tests/wAndNotThis/screen_shake/BossDamageShake.BossDamageShake_C" (`self.K2_GetActorLocation` (`GameplayStatics.GetPlayerPawn` 0)) 150.0 300.0))))))))

(event `PhysicalHitReact`
  ;[1 1 1] Physical animation
  (`SkeletalMeshComponent.SetAllBodiesBelowPhysicsBlendWeight` (`self.Mesh`) (`self.BoneName`) (`self.Physics Blend Weight`) false false)
  (`PhysicalAnimationComponent.ApplyPhysicalAnimationProfileBelow` (`self.PhysicalAnimation`) (`self.BoneName`) "DamagePhysics" true false))

(fn `UserConstructionScript`)