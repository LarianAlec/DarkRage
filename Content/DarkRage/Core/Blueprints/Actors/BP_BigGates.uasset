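; BP_BigGates is a large gate actor that opens when its OpenGate event is called.
; A one-time IsOpened check starts a timeline that animates the Root component's relative Z location.
; When the timeline finishes, it marks the gate as opened and asks GM_DarkRageCharacter_Actual to show the open-gates text in the HUD.
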(event `self.OpenGate`
  (if (not (`self.IsOpened`))
    (bind (_direction _zlocaltransform) (`Timeline|ZTransform` :!via `PlayFromStart`)
      (:`Update`
        (`SceneComponent.K2_SetRelativeLocation` (`self.Root`) (`KismetMathLibrary.MakeVector` 0.0 0.0 _zlocaltransform) false false))
      (:`Finished`
        (set `self.IsOpened` true)
        ;[1 1 1] Show in HUD OpenGates_TextBlock
        (bind _asgm_dark_rage_character_actual (cast `/Game/DarkRage/Core/Blueprints/GameModes/GM_DarkRageCharacter_Actual` (`GameplayStatics.GetGameMode`)))
        (`/Game/DarkRage/Core/Blueprints/GameModes/GM_DarkRageCharacter_Actual.ShowTextBlockInHUD_OpenGates` _asgm_dark_rage_character_actual)))))

(fn `UserConstructionScript`
  (`parent.UserConstructionScript`))