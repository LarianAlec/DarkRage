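; Enemy AI character that patrols, spots the player and dies from damage.
; On first seeing the player through PawnSensing, it writes the target to the blackboard, fires PlayerSpotted and switches to a randomized chase speed.
; It also alerts nearby unwarned enemies by sphere overlap, setting their speed, blackboard state and target.
; Damage is multiplied for headshots; death fires Died, ragdolls the mesh with a radial impulse and destroys the actor after a delay.
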(event `self.ReceiveBeginPlay`
  ;[0.6094 0 0.3659 1 30] Initialization StartLocation && Speed
  (set `self.StartLocation` (`self.K2_GetActorLocation`))
  (`self.UpdateSpeed` (`self.PatrolSpeed`)))

(event `/Game/UEGameCode/Core/Interfaces/BPI_Damage.ReceiveDamage`
  (params (Damage :type "Float (double-precision)") (ImpactLocation :type "Vector Structure") (HitBoneName :type Name))
  (bind _mesh (`self.Mesh`))
  ;[0.3333 0.02491 0 1 30] Apply Damage and Death
  (bind _output_get (set `self.Health` (- (`self.Health`) (* Damage (`KismetMathLibrary.SelectFloat` 5.0 1.0 (== HitBoneName "head"))))))
  (if (<= _output_get 0.0)
    (`/Engine/EditorBlueprintResources/StandardMacros.DoOnce` false
      (:`Completed`
        (`self.OnDied`)
        (`PrimitiveComponent.SetCollisionEnabled` _mesh "PhysicsOnly")
        (`PrimitiveComponent.SetSimulatePhysics` _mesh true)
        (`PrimitiveComponent.AddRadialImpulse` _mesh ImpactLocation 25.0 1000.0 "RIF_Constant" true)
        (`PrimitiveComponent.SetCollisionEnabled` (`self.CapsuleComponent`) "PhysicsOnly")
        (`KismetSystemLibrary.Delay` 10.0)
        (`self.K2_DestroyActor`)))))

(event `self.PawnSensing.OnSeePawn`
  (params (Pawn :type "Pawn Object Reference"))
  (bind (_aicontroller_blackboard _initializated_keyname) (`self.Initializate BB Data` "Enemy"))
  ;[0.4445 0.3698 1] On See Player
  (if (== Pawn (`GameplayStatics.GetPlayerCharacter` 0))
    (`self.EnemyRef`
      (:`then`)
      (:`else`
        (bind _output_get (set `self.EnemyRef` Pawn))
        (`BlackboardComponent.SetValueAsObject` _aicontroller_blackboard _initializated_keyname _output_get)
        (`self.PlayerSpotted`)
        (`|ExecutionSequence`
          (:`then_0`
            (if (not (`self.IsWarned`))
              (`self.WarnFriends`)))
          (:`then_1`
            (`self.WarnAI`)))))))

(event `WarnAI`
  (set `self.IsWarned` true)
  (`self.UpdateSpeed` (`KismetMathLibrary.RandomFloatInRange` 300.0 (`self.ChaseSpeed`))))

(fn `Initializate BB Data`
  (params (KeyName :type Name))
  (returns (AIController_Blackboard :type "BlackboardComponent Object Reference") (Initializated_KeyName :type Name))
  (return (`AIBlueprintHelperLibrary.GetBlackboard` (`AIBlueprintHelperLibrary.GetAIController` self)) (`KismetSystemLibrary.MakeLiteralName` KeyName)))

(fn `UpdateSpeed`
  (params (Speed :type "Float (double-precision)"))
  (set `CharacterMovementComponent.MaxWalkSpeed` Speed (`self.CharacterMovement`)))

(fn `UserConstructionScript`)

(fn `WarnFriends`
  (locals (Fiend :type "/Game/UEGameCode/Core/AI/BP_AI_Enemy Object Reference"))
  (bind _returnvalue (`AIBlueprintHelperLibrary.GetBlackboard` (`AIBlueprintHelperLibrary.GetAIController` (`local.Fiend`))))
  (bind _outactors (`KismetSystemLibrary.SphereOverlapActors` (`SceneComponent.K2_GetComponentLocation` (`self.CapsuleComponent`)) 1500.0 (`|MakeArray` "ObjectTypeQuery3" :!type "EObjectTypeQuery Enum") "BP_AI_Enemy_C"))
  (for _array_element _outactors
    (bind _asbp_ai_enemy (cast `/Game/UEGameCode/Core/AI/BP_AI_Enemy` _array_element))
    (set `local.Fiend` _asbp_ai_enemy)
    (if (not (`/Game/UEGameCode/Core/AI/BP_AI_Enemy.IsWarned` (`local.Fiend`)))
      (`self.WarnAI` (`local.Fiend`))
      (`BlackboardComponent.SetValueAsEnum` _returnvalue "AIState" 3)
      (`BlackboardComponent.SetValueAsObject` _returnvalue "Enemy" (`GameplayStatics.GetPlayerCharacter` 0))
      (`self.PlayerSpotted` (`local.Fiend`)))))