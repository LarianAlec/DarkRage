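; Berserker AI character test Blueprint that handles its axe, default attack and damage, firing dispatchers for AI logic to follow.
; Equip and unequip montages use notifies to spawn the axe onto a hand socket or destroy it.
; A custom damage event multiplies head hits fivefold and subtracts from Health.
; Its death branch, as wired, runs once when Health is zero or above, ragdolling with an impact impulse before delayed destruction.
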(event `self.ReceiveBeginPlay`)

(event `self.AttackDefault`
  (`|PlayMontage` (`self.Mesh`) "/Game/AI_Tests_Tests/BossAnimationsPack/AI/AI_Berserk/Animation_Berserk/Sword_Anim_Pack/02_Attack/05_Combo_Attack_Wave_05/Combo_Attack_Wave_05_All_Seq_Montage.Combo_Attack_Wave_05_All_Seq_Montage"
    (:`OnCompleted`
      _)
    (:`OnInterrupted`
      _))
  (`self.On Attack End`))

(event `CustomEvent`
  (params (Damage :type "Float (double-precision)") (ImpactLocation :type "Vector Structure") (HitBoneName :type Name))
  (bind _mesh (`self.Mesh`))
  ;[0.3333 0.02491 0 1 30] Apply Damage and Death
  (bind _output_get (set `self.Health` (- (`self.Health`) (* Damage (`KismetMathLibrary.SelectFloat` 5.0 1.0 (== HitBoneName "head"))))))
  (if (<= 0.0 _output_get)
    (`/Engine/EditorBlueprintResources/StandardMacros.DoOnce` false
      (:`Completed`
        (`self.OnDied`)
        (`PrimitiveComponent.SetCollisionEnabled` _mesh "PhysicsOnly")
        (`PrimitiveComponent.SetSimulatePhysics` _mesh true)
        (`PrimitiveComponent.AddRadialImpulse` _mesh ImpactLocation 25.0 1000.0 "RIF_Constant" true)
        (`PrimitiveComponent.SetCollisionEnabled` (`self.CapsuleComponent`) "PhysicsOnly")
        (`KismetSystemLibrary.Delay` 10.0)
        (`self.K2_DestroyActor`)))))

(event `self.EquipWeapon`
  ;[1 1 1] Equip Axe
  (set `self.IsWeildingWeapon` true)
  (bind _notifyname (`|PlayMontage` (`self.Mesh`) "/Game/AI_Tests_Tests/BossAnimationsPack/AI/AI_Berserk/Animation_Berserk/Sword_Anim_Pack/01_Idle/Idle_To_Combat.Idle_To_Combat")
    (:`OnCompleted`
      (`self.OnWealdAxe`))
    (:`OnNotifyBegin`
      (switch `name` _notifyname
        (:`HoldAxe`
          (bind _returnvalue (`|SpawnActorFromClass` "/Game/AI_Tests_Tests/BossAnimationsPack/AI/Weapon_AI/Berserk/BB_Weapon_Axe_Berserk.BB_Weapon_Axe_Berserk_C" (`self.GetTransform`) "Undefined" "MultiplyWithRoot" null null))
          (bind _output_get (set `self.WeaponActor` _returnvalue))
          (`self.K2_AttachToComponent` _output_get (`self.Mesh`) "hand_r_Axe" "SnapToTarget" "SnapToTarget" "SnapToTarget" true))))))

(event `self.UnequipWeapon`
  ;[1 1 1] Unequip Axe
  (bind _notifyname (`|PlayMontage` (`self.Mesh`) "/Game/AI_Tests_Tests/BossAnimationsPack/AI/AI_Berserk/Animation_Berserk/Sword_Anim_Pack/01_Idle/Combat_To_Idle.Combat_To_Idle")
    (:`then`
      (`self.OnSheathAxe`))
    (:`OnNotifyBegin`
      (switch `name` _notifyname
        (:`DropAxe`
          (`self.K2_DestroyActor` (`self.WeaponActor`))
          (set `self.IsWeildingWeapon` false))))))

(fn `Initializate BB Data`
  (params (KeyName :type Name))
  (returns (AIController_Blackboard :type "BlackboardComponent Object Reference") (Initializated_KeyName :type Name))
  (return (`AIBlueprintHelperLibrary.GetBlackboard` (`AIBlueprintHelperLibrary.GetAIController` self)) (`KismetSystemLibrary.MakeLiteralName` KeyName)))

(fn `UserConstructionScript`
  (`parent.UserConstructionScript`))