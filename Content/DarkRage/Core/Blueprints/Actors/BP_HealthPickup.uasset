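; BP_HealthPickup is a health pickup actor that heals the player character on touch.
; A timeline started on BeginPlay moves the static mesh along a Z-axis curve to make it float.
; When a BP_DarkRageCharacter_Actual overlaps the sphere below max health, it heals by HealthValue, plays an apple-bite sound and destroys itself.
; At full health, the pickup stays in the world.
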(event `self.ReceiveBeginPlay`
  (bind (_direction _z_axis_movement) (`Timeline|FloatingAnim`)
    (:`Update`
      (`SceneComponent.K2_SetRelativeLocation` (`self.StaticMesh`) _z_axis_movement false false))))

(event `self.Sphere.OnComponentBeginOverlap`
  (params (OverlappedComponent :type "PrimitiveComponent Object Reference") (OtherActor :type "Actor Object Reference") (OtherComp :type "PrimitiveComponent Object Reference") (OtherBodyIndex :type Integer) (bFromSweep :type Boolean) (SweepResult :type "HitResult Structure (by ref)"))
  (bind _asbp_dark_rage_character_actual (cast `/Game/DarkRage/Core/Characters/DarkRageCharacter/BP_DarkRageCharacter_Actual` OtherActor))
  (bind _health (`/Game/DarkRage/Core/Blueprints/DamageSystem/BPI_DRDamageSystem.GetCurrentHelath` _asbp_dark_rage_character_actual))
  (bind _maxhealth (`/Game/DarkRage/Core/Blueprints/DamageSystem/BPI_DRDamageSystem.GetMaxHealth` _asbp_dark_rage_character_actual))
  (if (< _health _maxhealth)
    (`/Game/DarkRage/Core/Blueprints/DamageSystem/BPI_DRDamageSystem.Heal` _asbp_dark_rage_character_actual (`self.HealthValue`))
    (`GameplayStatics.PlaySound2D` "/Game/DarkRage/Core/SFX/Pickups/A_AppleBite_Cue.A_AppleBite_Cue" 1.0 1.0 0.0 null null)
    (`self.K2_DestroyActor`)))

(fn `UserConstructionScript`)