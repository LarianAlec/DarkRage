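; Berserker enemy AI pawn that fights with an axe, spawned onto its hand socket and destroyed again by equip and unequip montage notifies.
; Point damage is reported to AI perception and subtracted from BPCEnemy health, with 5x headshots and a HealthMult raised once health is below half.
; Death ragdolls the mesh with an impulse, makes noise and destroys the actor after a delay.
; A health bar widget rotates toward the camera each tick.
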(event `/Game/AI_Tests_Tests/BossAnimationsPack/AI/AI_Enemy_Base/BPI_Enemy.AttackDefault`)

(event `self.ReceiveTick`
  (params (DeltaSeconds :type "Float (single-precision)"))
  (bind _w_healthbar (`self.W_HealthBar`))
  ;[1 1 1] event tick on updata widjet rotation
  (`parent.ReceiveTick` DeltaSeconds)
  (`SceneComponent.K2_SetWorldRotation` _w_healthbar (`KismetMathLibrary.FindLookAtRotation` (`SceneComponent.K2_GetComponentLocation` _w_healthbar) (`SceneComponent.K2_GetComponentLocation` (`PlayerCameraManager.TransformComponent` (`GameplayStatics.GetPlayerCameraManager` 0)))) false false))

(event `self.ReceiveBeginPlay`
  (bind _pawnhealth (`self.PawnHealth`))
  (bind _bpc_enemy (`self.BPC_Enemy`))
  (set `/Game/AI_Tests_Tests/BossAnimationsPack/AI/AI_Enemy_Base/BPC_Enemy.Health` _pawnhealth _bpc_enemy)
  (set `/Game/AI_Tests_Tests/BossAnimationsPack/AI/AI_Enemy_Base/BPC_Enemy.MaxHealth` _pawnhealth _bpc_enemy)
  (bind _returnvalue (`|CreateWidget` "/Game/AI_Tests_Tests/BossAnimationsPack/AI/AI_Enemy_Base/W_HealthBarAI.W_HealthBarAI_C" null self))
  (`WidgetComponent.SetWidget` (`self.W_HealthBar`) _returnvalue)
  (add `self.OnTakePointDamage` (delegate `OnTakePointDamage_Event`)))

(event `OnTakePointDamage_Event`
  (params (DamagedActor :type "Actor Object Reference") (Damage :type "Float (single-precision)") (InstigatedBy :type "Controller Object Reference") (HitLocation :type "Vector Structure") (FHitComponent :type "PrimitiveComponent Object Reference") (BoneName :type Name) (ShotFromDirection :type "Vector Structure") (DamageType :type "DamageType Object Reference") (DamageCauser :type "Actor Object Reference"))
  (bind _w_healthbar (`self.W_HealthBar`))
  (bind _bpc_enemy (`self.BPC_Enemy`))
  (bind _health (`/Game/AI_Tests_Tests/BossAnimationsPack/AI/AI_Enemy_Base/BPC_Enemy.Health` _bpc_enemy))
  ;[1 0.05098 0] Apply Damage And Death via c++
  ;[1 1 1] Widjet
  (`|ExecutionSequence`
    (:`then_0`
      (`SceneComponent.SetHiddenInGame` _w_healthbar true false)
      (`KismetSystemLibrary.Delay` 3.0)
      (`SceneComponent.SetHiddenInGame` _w_healthbar true false))
    (:`then_1`
      (`AISense_Damage.ReportDamageEvent` DamagedActor InstigatedBy Damage ShotFromDirection)
      (set `self.Hit Location` HitLocation)
      (set `self.Burst` (> (/ (`/Game/AI_Tests_Tests/BossAnimationsPack/AI/AI_Enemy_Base/BPC_Enemy.MaxHealth` _bpc_enemy) 2.0) _health))
      (`self.Burst Update`)
      (bind _output_get (set `/Game/AI_Tests_Tests/BossAnimationsPack/AI/AI_Enemy_Base/BPC_Enemy.Health` (- _health (* (* Damage (`KismetMathLibrary.SelectFloat` 5.0 1.0 (== BoneName "head"))) (`self.HealthMult`))) _bpc_enemy))
      (if (<= _output_get 0.0)
        (`self.Died`)))))

(event `Burst Update`
  (if (`self.Burst`)
    (set `self.HealthMult` 2.0)))

(event `Died`
  (bind _mesh (`self.Mesh`))
  (bind _weaponactor (`self.WeaponActor`))
  ;[0.3229 0.3229 0.3229] Death
  (`self.OnDied`)
  (`PrimitiveComponent.SetCollisionEnabled` _mesh "PhysicsOnly")
  (`PrimitiveComponent.SetSimulatePhysics` _mesh true)
  (`PrimitiveComponent.AddRadialImpulse` _mesh (`self.Hit Location`) 25.0 1000.0 "RIF_Constant" true)
  (`PrimitiveComponent.SetCollisionEnabled` (`self.CapsuleComponent`) "PhysicsOnly")
  (`SceneComponent.SetHiddenInGame` (`self.W_HealthBar`) true false)
  ;[1 1 1] Noise of reaper
  (`self.MakeNoise` 1.0 self (`self.K2_GetActorLocation`))
  (`KismetSystemLibrary.Delay` 10.0)
  (`self.K2_DestroyActor`)
  (if (`KismetSystemLibrary.IsValid` _weaponactor)
    (`self.K2_DestroyActor` _weaponactor)))

(event `/Game/AI_Tests_Tests/BossAnimationsPack/AI/AI_Enemy_Base/BPI_Enemy.EquipWeapon`
  ;[1 1 1] Equip Axe
  (set `self.IsWeildingWeapon` true)
  (bind _notifyname (`|PlayMontage` (`self.Mesh`) "/Game/AI_Tests_Tests/BossAnimationsPack/AI/AI_Berserk/Animation_Berserk/Sword_Anim_Pack/01_Idle/Idle_To_Combat.Idle_To_Combat")
    (:`OnCompleted`
      (`self.OnWealdAxe`))
    (:`OnNotifyBegin`
      (switch `name` _notifyname
        (:`HoldAxe`
          (bind _returnvalue (`|SpawnActorFromClass` "/Game/AI_Tests_Tests/BossAnimationsPack/AI/Weapon_AI/Berserk/BB_Weapon_Axe_Berserk.BB_Weapon_Axe_Berserk_C" (`self.GetTransform`) "Undefined" "MultiplyWithRoot" null null))
          (bind _output_get (set `self.WeaponActor` _returnvalue))
          (`self.K2_AttachToComponent` _output_get (`self.Mesh`) "hand_r_Axe" "SnapToTarget" "SnapToTarget" "SnapToTarget" true))))))

(event `/Game/AI_Tests_Tests/BossAnimationsPack/AI/AI_Enemy_Base/BPI_Enemy.UnequipWeapon`
  (bind _weaponactor (`self.WeaponActor`))
  ;[1 1 1] Unequip Axe
  (set `self.IsWeildingWeapon` false)
  (bind _notifyname (`|PlayMontage` (`self.Mesh`) "/Game/AI_Tests_Tests/BossAnimationsPack/AI/AI_Berserk/Animation_Berserk/Sword_Anim_Pack/01_Idle/Combat_To_Idle.Combat_To_Idle")
    (:`then`
      (`self.OnSheathAxe`))
    (:`OnNotifyBegin`
      (switch `name` _notifyname
        (:`DropAxe`
          (if (`KismetSystemLibrary.IsValid` _weaponactor)
            (`self.K2_DestroyActor` _weaponactor)))))))

(event `/Game/UEGameCode/Core/Interfaces/BPI_Damage.ReceiveDamage`
  (params (Damage :type "Float (double-precision)") (ImpactLocation :type "Vector Structure") (HitBoneName :type Name))
  ;[0.3333 0.02491 0 1 30] Apply Damage and Death (old)
)

(fn `Get CurrentHealth`
  (returns (Health :type "Float (double-precision)"))
  (return (`/Game/AI_Tests_Tests/BossAnimationsPack/AI/AI_Enemy_Base/BPC_Enemy.Health` (`self.BPC_Enemy`))))

(fn `Get MaxHealth`
  (returns (MaxHealth :type "Float (double-precision)"))
  (return (`/Game/AI_Tests_Tests/BossAnimationsPack/AI/AI_Enemy_Base/BPC_Enemy.MaxHealth` (`self.BPC_Enemy`))))

(fn `UserConstructionScript`
  (`parent.UserConstructionScript`))