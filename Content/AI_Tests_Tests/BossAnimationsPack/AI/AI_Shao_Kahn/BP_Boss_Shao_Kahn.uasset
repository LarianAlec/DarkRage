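; Boss character Shao Kahn for an AI test, with health, death and axe equip logic.
; Point damage lowers Health with a headshot multiplier; at zero it fires a died event, ragdolls with an impulse at the hit, makes noise, then destroys itself and its weapon.
; Equip and unequip montages use notifies to spawn the weapon on the Staff socket or destroy it, and fire wield and sheathe dispatchers.
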(event `self.ReceiveBeginPlay`
  (add `self.OnTakePointDamage` (delegate `OnTakePointDamage_Event`)))

(event `OnTakePointDamage_Event` :!signature `self.OnTakePointDamage`
  (params (DamagedActor :type "Actor Object Reference") (Damage :type "Float (single-precision)") (InstigatedBy :type "Controller Object Reference") (HitLocation :type "Vector Structure") (FHitComponent :type "PrimitiveComponent Object Reference") (BoneName :type Name) (ShotFromDirection :type "Vector Structure") (DamageType :type "DamageType Object Reference") (DamageCauser :type "Actor Object Reference"))
  (bind _mesh (`self.Mesh`))
  ;[1 0.05098 0] Apply Damage And Death via c++
  (bind _output_get (set `self.Health` (- (`self.Health`) (* Damage (`KismetMathLibrary.SelectFloat` 5.0 1.0 (== BoneName "head"))))))
  (if (<= _output_get 0.0)
    (`/Engine/EditorBlueprintResources/StandardMacros.DoOnce` false
      (:`Completed`
        (`self.OnDied`)
        (`PrimitiveComponent.SetCollisionEnabled` _mesh "PhysicsOnly")
        (`PrimitiveComponent.SetSimulatePhysics` _mesh true)
        (`PrimitiveComponent.AddRadialImpulse` _mesh HitLocation 25.0 1000.0 "RIF_Constant" true)
        (`PrimitiveComponent.SetCollisionEnabled` (`self.CapsuleComponent`) "PhysicsOnly")
        ;[1 1 1] Noise of reaper
        (`self.MakeNoise` 1.0 self (`self.K2_GetActorLocation`))
        (`KismetSystemLibrary.Delay` 10.0)
        (`self.K2_DestroyActor`)
        (`self.K2_DestroyActor` (`self.WeaponActor`))))))

(event `/Game/AI_Tests_Tests/BossAnimationsPack/AI/AI_Berserk/BPI_Berserk.EquipWeapon`
  ;[1 1 1] Equip Axe
  (set `self.IsWeildingWeapon` true)
  (bind _notifyname (`|PlayMontage` (`self.Mesh`) "/Game/AI_Tests_Tests/BossAnimationsPack/AI/AI_Berserk/Animation_Berserk/Sword_Anim_Pack/01_Idle/Idle_To_Combat.Idle_To_Combat")
    (:`OnCompleted`
      (`self.OnWealdAxe`))
    (:`OnNotifyBegin`
      (switch `name` _notifyname
        (:`HoldAxe`
          (bind _returnvalue (`|SpawnActorFromClass` "/Game/AI_Tests_Tests/BossAnimationsPack/AI/Weapon_AI/Shao_Kahn/BB_Weapon_Shao_Kahn.BB_Weapon_Shao_Kahn_C" (`self.GetTransform`) "Undefined" "MultiplyWithRoot" null null))
          (bind _output_get (set `self.WeaponActor` _returnvalue))
          (`self.K2_AttachToComponent` _output_get (`self.Mesh`) "Staff" "SnapToTarget" "SnapToTarget" "SnapToTarget" true))))))

(event `/Game/AI_Tests_Tests/BossAnimationsPack/AI/AI_Berserk/BPI_Berserk.UnequipWeapon`
  ;[1 1 1] Unequip Axe
  (bind _notifyname (`|PlayMontage` (`self.Mesh`) "/Game/AI_Tests_Tests/BossAnimationsPack/AI/AI_Berserk/Animation_Berserk/Sword_Anim_Pack/01_Idle/Combat_To_Idle.Combat_To_Idle")
    (:`then`
      (`self.OnSheathAxe`))
    (:`OnNotifyBegin`
      (switch `name` _notifyname
        (:`DropAxe`
          ;;[1 1 1] Fix -> not valid if not spawn
          (`self.K2_DestroyActor` (`self.WeaponActor`))
          (set `self.IsWeildingWeapon` false))))))

(fn `UserConstructionScript`
  (`parent.UserConstructionScript`))