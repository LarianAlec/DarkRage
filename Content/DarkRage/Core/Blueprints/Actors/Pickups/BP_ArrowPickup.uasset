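; Arrow ammo pickup that a BP_DarkRageCharacter_Actual collects by overlapping its sphere.
; On overlap it adds AmountAmmo arrows through the character's equipment component and plays an attenuated pickup sound at its location.
; It then triggers the take-ammo animation on player 0's HUD and destroys itself.
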(event `self.ReceiveBeginPlay`)

(event `self.Sphere.OnComponentBeginOverlap`
  (params (OverlappedComponent :type "PrimitiveComponent Object Reference") (OtherActor :type "Actor Object Reference") (OtherComp :type "PrimitiveComponent Object Reference") (OtherBodyIndex :type Integer) (bFromSweep :type Boolean) (SweepResult :type "HitResult Structure (by ref)"))
  (bind _asbp_dark_rage_character_actual (cast `/Game/DarkRage/Core/Characters/DarkRageCharacter/BP_DarkRageCharacter_Actual` OtherActor))
  (`CharacterEquipmentComponent.AddBullets` (`DRBaseCharacter.CharacterEquipmentComponent` _asbp_dark_rage_character_actual) "Arrows" (`self.AmountAmmo`))
  (`GameplayStatics.SpawnSoundAtLocation` "/Game/DarkRage/Core/SFX/Pickups/A_ArrowPickup_Cue.A_ArrowPickup_Cue" (`self.K2_GetActorLocation`) (struct) 1.0 1.0 0.0 "/Game/DarkRage/Core/SFX/EnemyMelee/ATT_Melee.ATT_Melee" null)
  (`|ExecutionSequence`
    (:`then_0`
      (bind _asbp_dark_rage_hud (cast `/Game/DarkRage/Core/Blueprints/HUD/BP_DarkRage_HUD` (`PlayerController.GetHUD` (`GameplayStatics.GetPlayerController` 0))))
      (`/Game/DarkRage/Core/Blueprints/HUD/BP_DarkRage_HUD.PlayTakeAmmoAnimtionInUI` _asbp_dark_rage_hud))
    (:`then_1`
      (`self.K2_DestroyActor`))))

(fn `UserConstructionScript`)