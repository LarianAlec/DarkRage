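; Master Blueprint for a flocking point boundary box, a placeable tool actor that marks a configurable volume, presumably for bird flocking.
; Its construction script sizes the Box component from the three flocking volume dimensions and toggles whether it shows in game.
; It also sets the editor Billboard's sprite and vertical offset.
; The event graph holds only disabled placeholder events, so the actor has no runtime logic of its own.
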(fn `UserConstructionScript`
  (`BoxComponent.SetBoxExtent` (`self.Box`) (`KismetMathLibrary.MakeVector` (`self.FlockingVolumeX`) (`self.FlockingVolumeY`) (`self.FlockingVolumeZ`)) true)
  (`SceneComponent.SetHiddenInGame` (`self.Box`) (not (`self.ShowBoxInGame`)) false)
  (`BillboardComponent.SetSprite` (`self.Billboard`) (`self.EditorBillboardSprite`))
  (`BillboardComponent.SetOpacityMaskRefVal` (`self.Billboard`) 1.0)
  (`SceneComponent.K2_SetRelativeLocation` (`self.Billboard`) (`KismetMathLibrary.MakeVector` 0.0 0.0 (`self.EditorBillboardOffsetZ`)) false false))