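; Start menu HUD that creates the background video, main, options and level-select widgets on BeginPlay.
; It shows the main menu first and sets UI-only input with a visible mouse cursor.
; Toggle events switch screens through ToggleWidget, which collapses the active widget, shows the requested one and tracks it as active.
; The credits event instead opens the separate CreditsMenu_P level.
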(event `self.ReceiveBeginPlay`
  (bind _returnvalue (`GameplayStatics.GetPlayerController` 0))
  (bind _wbp_mainmenu (`self.WBP_MainMenu`))
  (`|ExecutionSequence`
    (:`then_0`
      ;[1 1 1] WBP_Torches
      (bind _returnvalue_2 (`|CreateWidget` "/Game/UI_Logic/Widgets/WBP_MAinMenuBackVideo.WBP_MAinMenuBackVideo_C"))
      (bind _output_get (set `self.WBP_Torches` _returnvalue_2))
      (`UserWidget.AddToViewport` _output_get 0)
      ;[1 1 1] WBP_MainMenu
      (bind _returnvalue_3 (`|CreateWidget` "/Game/UI_Logic/Widgets/WBP_MainMenu1.WBP_MainMenu1_C"))
      (bind _output_get_2 (set `self.WBP_MainMenu` _returnvalue_3))
      (`UserWidget.AddToViewport` _output_get_2 0)
      ;[1 1 1] WBP_OptionMenu
      (bind _returnvalue_4 (`|CreateWidget` "/Game/UI_Logic/Widgets/WBP_OptionMainMenu.WBP_OptionMainMenu_C"))
      (bind _output_get_3 (set `self.WBP_OptionMenu` _returnvalue_4))
      (`UserWidget.AddToViewport` _output_get_3 0)
      ;[1 1 1] WBP_LevelMenu
      (bind _returnvalue_5 (`|CreateWidget` "/Game/UI_Logic/Widgets/WBP_ChooseLVL.WBP_ChooseLVL_C"))
      (bind _output_get_4 (set `self.WBP_LevelMenu` _returnvalue_5))
      (`UserWidget.AddToViewport` _output_get_4 0))
    (:`then_1`
      (set `Widget.Visibility` "Visible" _wbp_mainmenu)
      (set `self.ActiveWidget` _wbp_mainmenu))
    (:`then_2`
      (`WidgetBlueprintLibrary.SetInputMode_UIOnlyEx` _returnvalue (`self.ActiveWidget`))
      (set `PlayerController.bShowMouseCursor` true _returnvalue))))

(event `ToggleOptionMenu`
  (`self.ToggleWidget` (`self.WBP_OptionMenu`)))

(event `ToggleMainMenu`
  (`self.ToggleWidget` (`self.WBP_MainMenu`)))

(event `ToggleLevelMenu`
  (`self.ToggleWidget` (`self.WBP_LevelMenu`)))

(event `ToggleCredits`
  (`GameplayStatics.OpenLevelBySoftObjectPtr` "/Game/DarkRage/Maps/StartMenu/CreditsMenu_P.CreditsMenu_P"))

(fn `ToggleWidget`
  (params (WidgetToFocus :type "UserWidget Object Reference"))
  (`Widget.SetVisibility` (`self.ActiveWidget`) "Collapsed")
  (`Widget.SetVisibility` WidgetToFocus "Visible")
  (set `self.ActiveWidget` WidgetToFocus))

(fn `UserConstructionScript`)