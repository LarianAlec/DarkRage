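; BP_StaticArcher is an archer enemy AI that fires projectile arrows at an attack target.
; Attack line-traces from the actor to just above the target, then spawns BP_EnemyArrow from the arrow socket toward that point, alongside the fire montage.
; Equip and unequip montage notifies attach or destroy the bow.
; BeginPlay seeds damage-system health and randomizes the mesh material; an older line-trace attack remains unconnected.
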(event `self.Attack`
  (params (AttackTarget :type "Actor Object Reference"))
  ;[1 0.01813 0] Projectile Attack
  (`parent.Attack` AttackTarget)
  (`|ExecutionSequence`
    (:`then_0`
      (set `self.CrosshairWorldLocation` (`self.K2_GetActorLocation`))
      (set `self.ImpactPoint` (+ (`self.K2_GetActorLocation` AttackTarget) (0.0 0.0 30.0))))
    (:`then_1`
      (bind _outhit (`KismetSystemLibrary.LineTraceSingle` (`self.CrosshairWorldLocation`) (`self.ImpactPoint`) "TraceTypeQuery4" false (`|MakeArray` self :!type "Actor Object Reference")))
      (bind (_bblockinghit _binitialoverlap _time _distance _location _impactpoint) (`GameplayStatics.BreakHitResult` _outhit))
      (if _bblockinghit
        (set `self.ImpactPoint` _impactpoint))
      (set `self.ArrowSpawnLocation` (.location (`SceneComponent.GetSocketTransform` (`self.Mesh`) "ArrowSocket" "RTS_World")))
      (set `self.ArrowSpawnRotation` (`KismetMathLibrary.MakeRotFromX` (- (`self.ImpactPoint`) (`self.ArrowSpawnLocation`)))))
    (:`then_2`
      (bind _returnvalue (`|SpawnActorFromClass` "/Game/DarkRage/Core/Weapons/EnemyBow/BP_EnemyArrow.BP_EnemyArrow_C" (`KismetMathLibrary.MakeTransform` (`self.ArrowSpawnLocation`) (`self.ArrowSpawnRotation`)) "Undefined" "MultiplyWithRoot" self self))
      (set `/Game/DarkRage/Core/Weapons/EnemyBow/BP_EnemyArrow.ArrowDamage` (`self.DamageAmount`) _returnvalue))
    (:`then_3`
      (`|PlayMontage` (`self.Mesh`) "/Game/DarkRage/Core/AI/Archer/Animations/Fire/AM_Archer_Primary_Fire_Slow.AM_Archer_Primary_Fire_Slow"
        (:`then`
          (`self.OnAttackStarted`)
          (`GameplayStatics.SpawnSoundAtLocation` "/Game/DarkRage/Core/SFX/Bow/A_BowShoot_Cue.A_BowShoot_Cue" (`self.K2_GetActorLocation`) (struct) 1.0 1.0 0.0 "/Game/DarkRage/Core/SFX/Bow/ATT_BowShoot.ATT_BowShoot" null))
        (:`OnCompleted`
          (`/Game/DarkRage/Core/AI/Character/Interfaces/BPI_AICharacter.AttackEnd` AttackTarget :!label _label))
        (:`OnInterrupted`
          (goto _label))))))

(event `self.EquipWeapon`
  ;[1 0.4167 0] Equip Weapon
  (if (not (`self.IsArmed`))
    (bind _notifyname (`|PlayMontage` (`self.Mesh`) "/Game/DarkRage/Core/AI/Archer/Animations/Equip/AM_Archer_Equip.AM_Archer_Equip")
      (:`then`
        (`self.OnEquipWeaponStart`))
      (:`OnCompleted`
        (`self.OnEquipWeaponEnd` :!label _label_2))
      (:`OnInterrupted`
        (goto _label_2))
      (:`OnNotifyBegin`
        (switch `name` _notifyname
          (:`AttachWeaponToSocket`
            (bind _returnvalue (`|SpawnActorFromClass` "/Game/DarkRage/Core/Weapons/EnemyBow/BP_EnemyBow.BP_EnemyBow_C" (`self.GetTransform`) "Undefined" "MultiplyWithRoot" null null))
            (bind _output_get (set `self.WeaponActor` _returnvalue))
            (`self.K2_AttachToComponent` _output_get (`self.Mesh`) "LHandBowSocket" "SnapToTarget" "SnapToTarget" "SnapToTarget" true)
            (set `self.IsArmed` true)))))))

(event `self.UnequipWeapon`
  ;[1 0.4167 0] Unequip Weapon
  (if (`self.IsArmed`)
    (bind _notifyname (`|PlayMontage` (`self.Mesh`) "/Game/DarkRage/Core/AI/Archer/Animations/Equip/AM_Archer_Unequip.AM_Archer_Unequip")
      (:`then`
        (`self.OnUnequipWeaponStart`))
      (:`OnCompleted`
        (`self.OnUnequipWeaponEnd` :!label _label_3)
        (set `self.IsArmed` false))
      (:`OnInterrupted`
        (goto _label_3))
      (:`OnNotifyBegin`
        (switch `name` _notifyname
          (:`DetachWeaponFromSocket`
            (`self.K2_DestroyActor` (`self.WeaponActor`))))))))

(event `self.ReceiveAnyDamage`
  (params (Damage :type "Float (single-precision)") (DamageType :type "DamageType Object Reference") (InstigatedBy :type "Controller Object Reference") (DamageCauser :type "Actor Object Reference"))
  (`parent.ReceiveAnyDamage` Damage DamageType InstigatedBy DamageCauser))

(event `self.ReceiveBeginPlay`
  (bind _bpc_drdamagesystem (`self.BPC_DRDamageSystem`))
  (bind _health (`self.Health`))
  (`parent.ReceiveBeginPlay`)
  (set `/Game/DarkRage/Core/Blueprints/DamageSystem/BPC_DRDamageSystem.Health` _health _bpc_drdamagesystem)
  (set `/Game/DarkRage/Core/Blueprints/DamageSystem/BPC_DRDamageSystem.MaxHealth` _health _bpc_drdamagesystem)
  (`PrimitiveComponent.SetMaterial` (`self.Mesh`) 0 (`KismetArrayLibrary.Array_Random` (`self.MeshMaterialArray`))))

(fn `GetIdealRange`
  (returns (AttackRadius :type "Float (double-precision)") (DefendRadius :type "Float (double-precision)"))
  (return (`self.AttackRadius`) 600.0))

(fn `SetMovementSpeed`
  (params (NewSpeed :type "/Game/DarkRage/Core/AI/Character/Enums/E_MovementAISpeed Enum" :default "NewEnumerator0"))
  (returns (CurrentSpeed :type "Float (double-precision)"))
  (bind _output_get (set `CharacterMovementComponent.MaxWalkSpeed` (select `/Game/DarkRage/Core/AI/Character/Enums/E_MovementAISpeed` NewSpeed :`NewEnumerator1` (`self.WalkingSpeed`) :`NewEnumerator4` (`self.StrafingSpeed`) :`NewEnumerator2` (`self.JoggingSpeed`) :`NewEnumerator3` (`self.SprintingSpeed`)) (`self.CharacterMovement`)))
  (return _output_get))

(fn `UserConstructionScript`
  (`parent.UserConstructionScript`))