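; BP_Enemy is a base AI enemy character exposing patrol route, movement speed, attack status and health/armor queries, with the health, armor and attack getters returning stub values.
; SetMovementSpeed maps a speed state to MaxWalkSpeed, and AgroStateEvent toggles the aggro flag.
; JumptoDestination launches the character along a suggested projectile arc to a target point.
; Calm/combat music logic driven by blackboard state and GameMode flags is disconnected and never runs.
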(event `self.ReceiveBeginPlay`)

(event `self.ReceiveTick`
  (params (DeltaSeconds :type "Float (single-precision)")))

(event `AgroStateEvent`
  (set `self.AgroState` (not (`self.AgroState`))))

(event `/Game/AI_Tests_Tests/BossAnimationsPack/AI/AI_Enemy_Base/BPI_Enemy.JumpToDestination`
  (params (Destination :type "Vector Structure"))
  (bind _outlaunchvelocity (`GameplayStatics.SuggestProjectileVelocity_CustomArc` (`self.K2_GetActorLocation`) (`KismetMathLibrary.MakeVector` (.x Destination) (.y Destination) (.z Destination))))
  (`self.LaunchCharacter` _outlaunchvelocity true true))

(fn `Get CurrentArmor`
  (returns (CurrentArmor :type "Float (double-precision)"))
  (return 0.0))

(fn `Get CurrentHealth`
  (returns (Health :type "Float (double-precision)"))
  (return 0.0))

(fn `Get MaxArmor`
  (returns (MaxArmor :type "Float (double-precision)"))
  (return 0.0))

(fn `Get MaxHealth`
  (returns (MaxHealth :type "Float (double-precision)"))
  (return 0.0))

(fn `GetPatrolRoute`
  (returns (PatrolRoute :type "/Game/AI_Tests_Tests/BossAnimationsPack/AI/AI_Berserk/BP_PatrolRoute Object Reference"))
  (return (`self.PatrolRouts`)))

(fn `IsAttacking`
  (returns (Attacking :type Boolean))
  (return false))

(fn `SetMovementSpeed`
  (params (Speed :type "/Game/AI_Tests_Tests/BossAnimationsPack/AI/BehaviourTrees/Enums/E_MovementSpeed Enum" :default "NewEnumerator0"))
  (returns (SpeedValue :type "Float (double-precision)"))
  (bind _output_get (set `CharacterMovementComponent.MaxWalkSpeed` (select `/Game/AI_Tests_Tests/BossAnimationsPack/AI/BehaviourTrees/Enums/E_MovementSpeed` Speed :`NewEnumerator1` 200.0 :`NewEnumerator2` 300.0 :`NewEnumerator3` 600.0 :`NewEnumerator4` 800.0 :!type "Float (single-precision)") (`self.CharacterMovement`)))
  (return _output_get))

(fn `UserConstructionScript`)