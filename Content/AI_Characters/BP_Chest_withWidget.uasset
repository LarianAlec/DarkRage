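; Chest actor Blueprint with a "HITME" widget component that billboards toward the player camera.
; BeginPlay creates a WBP_Chest_HITME instance and stores it, then, only when WidgetHide is true, unhides the Widget component and calls the parent BeginPlay.
; While WidgetHide is true, Tick rotates the widget to look at the first player's camera.
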(event `self.ReceiveBeginPlay`
  (bind _returnvalue (`|CreateWidget` "/Game/AI_Characters/WBP_Chest_HITME.WBP_Chest_HITME_C"))
  (set `self.Widgets` _returnvalue)
  (if (`self.WidgetHide`)
    (`SceneComponent.SetHiddenInGame` (`self.Widget`) false false)
    (`parent.ReceiveBeginPlay`)))

(event `self.ReceiveTick`
  (params (DeltaSeconds :type "Float (single-precision)"))
  (bind _widget (`self.Widget`))
  (if (`self.WidgetHide`)
    (`SceneComponent.K2_SetWorldRotation` _widget (`KismetMathLibrary.FindLookAtRotation` (`SceneComponent.K2_GetComponentLocation` _widget) (`SceneComponent.K2_GetComponentLocation` (`PlayerCameraManager.TransformComponent` (`GameplayStatics.GetPlayerCameraManager` 0)))) false false)))

(fn `UserConstructionScript`
  (`parent.UserConstructionScript`))