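; Game mode for DarkRage that provides events for arena encounters and their music.
; One event shows markers above actors tagged ArenaEnemy, trying BP_AICharacter first and falling back to BP_Enemy.
; Another tells the HUD's arena counter widget to show its open-gates text.
; Two music events stop the current track and spawn either calm ambient or arena music as 2D sound, storing it as CurrentMusic.
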(event `ShowArenaMarkerAboveEnemy`
  (bind _outactors (`GameplayStatics.GetAllActorsWithTag` "ArenaEnemy"))
  (for _array_element _outactors
    (bind _asbp_aicharacter (cast `/Game/DarkRage/Core/AI/Character/BP_AICharacter` _array_element)
      (:`then`
        (`/Game/DarkRage/Core/AI/Character/BP_AICharacter.ShowArenaMarker` _asbp_aicharacter))
      (:`CastFailed`
        (bind _asbp_enemy (cast `/Game/AI_Characters/AI_Enemy_Base/BP_Enemy` _array_element))
        (`/Game/AI_Characters/AI_Enemy_Base/BP_Enemy.ShowArenaMarker` _asbp_enemy)))))

(event `ShowTextBlockInHUD_OpenGates`
  (bind _asbp_dark_rage_hud (cast `/Game/DarkRage/Core/Blueprints/HUD/BP_DarkRage_HUD` (`PlayerController.GetHUD` (`GameplayStatics.GetPlayerController` 0))))
  (bind _wbp_arenacounter (`/Game/DarkRage/Core/Blueprints/HUD/BP_DarkRage_HUD.WBP_ArenaCounter` _asbp_dark_rage_hud)
    (:`then`
      (`/Game/UI_Logic/Widgets/WBP_ArenaCounter.ShowTextBlock_OpenGates` _wbp_arenacounter))
    (:`else`)))

(event `PlayCalmAmbient`
  (bind _currentmusic (`self.CurrentMusic`)
    (:`then`
      (`AudioComponent.Stop` _currentmusic))
    (:`else`
      _))
  (bind _returnvalue (`GameplayStatics.SpawnSound2D` (`self.AmbientMusic`) 1.0 1.0 0.0 null))
  (set `self.CurrentMusic` _returnvalue))

(event `PlayArenaMusic`
  (bind _currentmusic (`self.CurrentMusic`)
    (:`then`
      (`AudioComponent.Stop` _currentmusic))
    (:`else`
      _))
  (bind _returnvalue (`GameplayStatics.SpawnSound2D` (`self.ArenaMusic`) 1.0 1.0 0.0 null))
  (set `self.CurrentMusic` _returnvalue))

(fn `UserConstructionScript`)