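; Shield-and-axe AI enemy character with a camera-facing health bar that appears briefly when it is hit.
; Point damage lowers BPCEnemy health, doubled on head hits, reports a damage event, sets a timed Block flag and triggers AIDeath at zero health.
; Equip and unequip montage notifies spawn and socket-attach, or destroy, the axe and shield actors.
; Getters expose health and attack state.
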(event `self.ReceiveTick`
  (params (DeltaSeconds :type "Float (single-precision)"))
  (bind _w_healthbar (`self.W_HealthBar`))
  ;[1 1 1] event tick on updata widjet rotation
  (`parent.ReceiveTick` DeltaSeconds)
  (`SceneComponent.K2_SetWorldRotation` _w_healthbar (`KismetMathLibrary.FindLookAtRotation` (`SceneComponent.K2_GetComponentLocation` _w_healthbar) (`SceneComponent.K2_GetComponentLocation` (`PlayerCameraManager.TransformComponent` (`GameplayStatics.GetPlayerCameraManager` 0)))) false false))

(event `self.ReceiveBeginPlay`
  (bind _bpc_enemy (`self.BPC_Enemy`))
  (set `self.DeathMontage` "/Game/AI_Tests_Tests/BossAnimationsPack/AI_Characters/AI_Shield/AxeAndShield/Animations/InPlace/Death_IP_Montage.Death_IP_Montage")
  (bind _output_get (set `/Game/AI_Tests_Tests/BossAnimationsPack/AI_Characters/AI_Enemy_Base/BPC_Enemy.Health` (`self.PawnHealth`) _bpc_enemy))
  (set `/Game/AI_Tests_Tests/BossAnimationsPack/AI_Characters/AI_Enemy_Base/BPC_Enemy.MaxHealth` _output_get _bpc_enemy)
  (bind _returnvalue (`|CreateWidget` "/Game/AI_Tests_Tests/BossAnimationsPack/AI_Characters/AI_Enemy_Base/Bar_for_enemy/W_HealthBarAI.W_HealthBarAI_C" null self))
  (`WidgetComponent.SetWidget` (`self.W_HealthBar`) _returnvalue)
  (add `self.OnTakePointDamage` (delegate `OnTakePointDamage_Event`)))

(event `OnTakePointDamage_Event`
  (params (DamagedActor :type "Actor Object Reference") (Damage :type "Float (single-precision)") (InstigatedBy :type "Controller Object Reference") (HitLocation :type "Vector Structure") (FHitComponent :type "PrimitiveComponent Object Reference") (BoneName :type Name) (ShotFromDirection :type "Vector Structure") (DamageType :type "DamageType Object Reference") (DamageCauser :type "Actor Object Reference"))
  (bind _w_healthbar (`self.W_HealthBar`))
  (bind _bpc_enemy (`self.BPC_Enemy`))
  ;[1 0.05098 0] Apply Damage And Death via c++
  (`|ExecutionSequence`
    (:`then_0`
      ;[1 1 1] Widjet
      (`SceneComponent.SetHiddenInGame` _w_healthbar false false)
      (`KismetSystemLibrary.Delay` 5.0)
      (`SceneComponent.SetHiddenInGame` _w_healthbar true false))
    (:`then_1`
      (set `self.Block` true)
      (set `self.Hit Location` HitLocation)
      (bind _output_get (set `/Game/AI_Tests_Tests/BossAnimationsPack/AI_Characters/AI_Enemy_Base/BPC_Enemy.Health` (- (`/Game/AI_Tests_Tests/BossAnimationsPack/AI_Characters/AI_Enemy_Base/BPC_Enemy.Health` _bpc_enemy) (* Damage (`KismetMathLibrary.SelectFloat` 2.0 1.0 (== BoneName "head")))) _bpc_enemy))
      (`AISense_Damage.ReportDamageEvent` DamagedActor InstigatedBy Damage ShotFromDirection)
      (`|ExecutionSequence`
        (:`then_0`
          (`KismetSystemLibrary.Delay` 3.0)
          (set `self.Block` false))
        (:`then_1`
          (if (<= _output_get 0.0)
            (`self.Death`)))))))

(event `Death`
  ;[0.4948 0.4948 0.4948] Death
  (`SceneComponent.SetHiddenInGame` (`self.W_HealthBar`) true false)
  (bind _weaponactor_shield (`self.WeaponActor_Shield`)
    (:`then`
      (`self.AI_Death` _weaponactor_shield))
    (:`else`
      (`self.AI_Death` null))))

(event `/Game/AI_Tests_Tests/BossAnimationsPack/AI_Characters/AI_Enemy_Base/BPI_Enemy.EquipWeapon`
  ;[1 1 1] Equip Axe
  (set `self.IsWeildingWeapon` true)
  (bind _notifyname (`|PlayMontage` (`self.Mesh`) "/Game/AI_Tests_Tests/BossAnimationsPack/AI_Characters/AI_Shield/AxeAndShield/Animations/InPlace/Unequip_IP_Montage.Unequip_IP_Montage")
    (:`OnCompleted`
      (`self.OnWealdAxe`))
    (:`OnNotifyBegin`
      (switch `name` _notifyname
        (:`Axe`
          (bind _returnvalue (`|SpawnActorFromClass` "/Game/AI_Tests_Tests/BossAnimationsPack/AI_Characters/Weapon_AI/Axe_Shield/BP_Axe_Shield.BP_Axe_Shield_C" (`self.GetTransform`) "Undefined" "MultiplyWithRoot" null null))
          (bind _output_get (set `self.WeaponActor` _returnvalue))
          (`self.K2_AttachToComponent` _output_get (`self.Mesh`) "AxeSocket" "SnapToTarget" "SnapToTarget" "SnapToTarget" true))
        (:`Shield`
          (bind _returnvalue_2 (`|SpawnActorFromClass` "/Game/AI_Tests_Tests/BossAnimationsPack/AI_Characters/Weapon_AI/Axe_Shield/BP_Shield_Shield.BP_Shield_Shield_C" (`self.GetTransform`) "Undefined" "MultiplyWithRoot" null null))
          (bind _output_get_2 (set `self.WeaponActor_Shield` _returnvalue_2))
          (`self.K2_AttachToComponent` _output_get_2 (`self.Mesh`) "ShieldSocket" "SnapToTarget" "SnapToTarget" "SnapToTarget" true))))))

(event `/Game/AI_Tests_Tests/BossAnimationsPack/AI_Characters/AI_Enemy_Base/BPI_Enemy.UnequipWeapon`
  (bind _weaponactor (`self.WeaponActor`))
  (bind _weaponactor_shield (`self.WeaponActor_Shield`))
  ;[1 1 1] Unequip Axe
  (set `self.IsWeildingWeapon` false)
  (bind _notifyname (`|PlayMontage` (`self.Mesh`) "/Game/AI_Tests_Tests/BossAnimationsPack/AI_Characters/AI_Shield/AxeAndShield/Animations/InPlace/Sheathe_IP_Unequip.Sheathe_IP_Unequip")
    (:`then`
      (`self.OnSheathAxe`))
    (:`OnNotifyBegin`
      (switch `name` _notifyname
        (:`Axe`
          (if (`KismetSystemLibrary.IsValid` _weaponactor)
            (`self.K2_DestroyActor` _weaponactor)))
        (:`Shield`
          (if (`KismetSystemLibrary.IsValid` _weaponactor_shield)
            (`self.K2_DestroyActor` _weaponactor_shield)))))))

(fn `Get CurrentHealth`
  (returns (Health :type "Float (double-precision)"))
  (return (`/Game/AI_Tests_Tests/BossAnimationsPack/AI_Characters/AI_Enemy_Base/BPC_Enemy.Health` (`self.BPC_Enemy`))))

(fn `Get MaxHealth`
  (returns (MaxHealth :type "Float (double-precision)"))
  (return (`/Game/AI_Tests_Tests/BossAnimationsPack/AI_Characters/AI_Enemy_Base/BPC_Enemy.MaxHealth` (`self.BPC_Enemy`))))

(fn `IsAttacking`
  (returns (Attacking :type Boolean))
  (return (`self.Attackin`)))

(fn `UserConstructionScript`
  (`parent.UserConstructionScript`))