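; BP_AI_EnemyController is the AI controller that drives BP_AI_Enemy pawns through the BT_Enemy behavior tree.
; On possession it stores the pawn, binds to its death event, runs the tree, then seeds the blackboard with the pawn's start location, patrol range and patrol state.
; When the enemy dies, it stops the brain component's logic, halting the tree.
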(event `self.ReceivePossess`
  (params (PossessedPawn :type "Pawn Object Reference"))
  ;[1 0.248 0.2181] Bind StopBehaviorTree_Event to OnDie_EventDispatcher
  (bind _asbp_ai_enemy (cast `/Game/UEGameCode/Core/AI/BP_AI_Enemy` PossessedPawn))
  (bind _output_get (set `self.PawnRef` _asbp_ai_enemy))
  (add `/Game/UEGameCode/Core/AI/BP_AI_Enemy.OnDied` _output_get (delegate `StopBehaviorTree`))
  (`self.RunBehaviorTree` "/Game/UEGameCode/Core/AI/BT_Enemy.BT_Enemy")
  (`self.UpdateBBData`))

(event `StopBehaviorTree`
  ;[1 0.248 0.2181] Bind StopBehaviorTree_Event to OnDie_EventDispatcher
  (bind _braincomponent (`self.BrainComponent`)
    (:`then`
      (`BrainComponent.StopLogic` _braincomponent "Died")
      (`KismetSystemLibrary.PrintString` "Enemy Died"))
    (:`else`)))

(fn `InitializeBBData`
  (params (KeyName :type Name))
  (returns (AIControllerBlackboard :type "BlackboardComponent Object Reference") (InitializeKeyName :type Name))
  (return (`AIBlueprintHelperLibrary.GetBlackboard` self) KeyName))

(fn `UpdateBBData`
  (bind (_aicontrollerblackboard _initializekeyname) (`self.InitializeBBData` "StartLocation"))
  (bind (_aicontrollerblackboard_2 _initializekeyname_2) (`self.InitializeBBData` "PatrolRange"))
  (bind (_aicontrollerblackboard_3 _initializekeyname_3) (`self.InitializeBBData` "AIState"))
  (`BlackboardComponent.SetValueAsVector` _aicontrollerblackboard _initializekeyname (`/Game/UEGameCode/Core/AI/BP_AI_Enemy.StartLocation` (`self.PawnRef`)))
  (`BlackboardComponent.SetValueAsFloat` _aicontrollerblackboard_2 _initializekeyname_2 (`/Game/UEGameCode/Core/AI/BP_AI_Enemy.MaxPatrolDistance` (`self.PawnRef`)))
  (`BlackboardComponent.SetValueAsEnum` _aicontrollerblackboard_3 _initializekeyname_3 (`/Game/UEGameCode/Core/AI/BP_AI_Enemy.PatrolState` (`self.PawnRef`))))

(fn `UserConstructionScript`)