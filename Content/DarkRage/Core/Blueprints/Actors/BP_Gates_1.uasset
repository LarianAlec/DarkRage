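; BP_Gates_1 is an arena gate that opens once every actor tagged ArenaEnemy has died.
; On BeginPlay it counts those enemies, binds to each one's BPC_ArenaCounterComponent death event, and assigns an open-gate marker widget to its widget component.
; Each death decrements the count; at zero, after a short delay, a timeline yaw-rotates the door mesh and reveals the marker.
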(event `self.ReceiveBeginPlay`
  (`|ExecutionSequence`
    (:`then_0`
      (bind _outactors (`GameplayStatics.GetAllActorsWithTag` "ArenaEnemy"))
      (set `self.EnemiesCount` (`KismetArrayLibrary.Array_Length` _outactors))
      (for _array_element _outactors
        (bind _returnvalue (`self.FindComponentByTag` _array_element "/Game/DarkRage/Core/Blueprints/Components/BPC_ArenaCounterComponent.BPC_ArenaCounterComponent_C" "ArenaCounterComponent"))
        (`/Engine/EditorBlueprintResources/StandardMacros.IsValid` _returnvalue
          (:`Is Valid`
            (add `/Game/DarkRage/Core/Blueprints/Components/BPC_ArenaCounterComponent.OnDeath` _returnvalue (delegate `CheckEnemyCount`))))))
    (:`then_1`
      (bind _returnvalue_2 (`|CreateWidget` "/Game/DarkRage/UI/Widgets/WBP_OpenGateMarker.WBP_OpenGateMarker_C"))
      (`WidgetComponent.SetWidget` (`self.Widget`) _returnvalue_2))))

(event `CheckEnemyCount`
  (bind _result (`/Engine/EditorBlueprintResources/StandardMacros.DecrementInt` (`self.EnemiesCount`))
    (:`  `
      (if (== _result 0)
        (`KismetSystemLibrary.Delay` 1.0)
        (`self.OpenGate`)))))

(event `OpenGate`
  (if (not (`self.IsOpened`))
    (bind (_direction _zrotator) (`Timeline|DoorRotator` :!via `PlayFromStart`)
      (:`Update`
        (`SceneComponent.K2_SetRelativeRotation` (`self.SM_GateDoor`) (`KismetMathLibrary.MakeRotator` 0.0 0.0 _zrotator) false false)
        (`SceneComponent.SetHiddenInGame` (`self.Widget`) false false))
      (:`Finished`
        (set `self.IsOpened` true)))))

(fn `UserConstructionScript`)