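; BP_Chest is a damageable chest actor that is destroyed when its Health runs out.
; On BeginPlay it binds to OnTakePointDamage and subtracts incoming damage from Health, so only point damage is handled.
; At zero or below, Died broadcasts the OnDied dispatcher for any listeners, then destroys the actor.
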(event `self.ReceiveTick`
  (params (DeltaSeconds :type "Float (single-precision)")))

(event `self.ReceiveBeginPlay`
  (add `self.OnTakePointDamage` (delegate `OnTakePointDamage_Event`)))

(event `OnTakePointDamage_Event` :!signature `self.OnTakePointDamage`
  (params (DamagedActor :type "Actor Object Reference") (Damage :type "Float (single-precision)") (InstigatedBy :type "Controller Object Reference") (HitLocation :type "Vector Structure") (FHitComponent :type "PrimitiveComponent Object Reference") (BoneName :type Name) (ShotFromDirection :type "Vector Structure") (DamageType :type "DamageType Object Reference") (DamageCauser :type "Actor Object Reference"))
  (bind _output_get (set `self.Health` (- (`self.Health`) Damage)))
  (if (<= _output_get 0.0)
    (`self.Died`)))

(event `Died`
  (`self.OnDied`)
  (`self.K2_DestroyActor`))

(fn `UserConstructionScript`)