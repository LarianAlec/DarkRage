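; Base weapon Blueprint that gets its owning BP_DarkRageCharacter_LEGACY from the parent actor and sets its skeletal mesh on construction.
; Equip, stow, fire and reload events, including stop and cancel, are empty stubs.
; FireHitscan traces from the first-person camera within a spread cone, then from the muzzle toward that result with added random offset on hits, returning the second trace's hit.
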(event `self.ReceiveBeginPlay`
  ;[1 1 1] Get Player Reference
  (bind _asbp_dark_rage_character (cast `/Game/UEGameCode/Core/Blueprints/BP_DarkRageCharacter_LEGACY` (`self.GetParentActor`)))
  (set `self.PlayerRef` _asbp_dark_rage_character))

(event `Equip`
  ;[1 1 1] Events
)

(event `Stow`
  ;[1 1 1] Events
)

(event `Fire`
  ;[1 1 1] Events
)

(event `StopFire`
  ;[1 1 1] Events
)

(event `Reload`
  ;[1 1 1] Events
)

(event `CancelReload`
  ;[1 1 1] Events
)

(fn `Fire_Hitscan`
  (params (DrawDebug :type Boolean :default false))
  (returns (HitInfoL :type "HitResult Structure"))
  (locals (`Hit Info` :type "HitResult Structure"))
  (bind _first_person_camera_component (`/Game/UEGameCode/Core/Blueprints/BP_DarkRageCharacter_LEGACY.First Person Camera Component` (`self.PlayerRef`)))
  (bind _returnvalue (`SceneComponent.K2_GetComponentLocation` _first_person_camera_component))
  (bind _returnvalue_2 (`KismetMathLibrary.RandomUnitVectorInConeInDegrees` (`SceneComponent.GetForwardVector` _first_person_camera_component) (`self.Spread`)))
  ;[1 1 1] Trace From Center Screen to Max Weapon Range
  (bind (_outhit _returnvalue_3) (`KismetSystemLibrary.LineTraceSingle` _returnvalue (+ _returnvalue (* _returnvalue_2 (`self.Range`))) "TraceTypeQuery1" false (`|MakeArray` (`self.PlayerRef`) :!type "Actor Object Reference")))
  ;[1 1 1] Trace From Weapon Muzzle to Center Trace Hit Location
  (set `local.Hit Info` _outhit)
  (bind (_bblockinghit _binitialoverlap _time _distance _location _impactpoint _normal _impactnormal _physmat _hitactor _hitcomponent _hitbonename _bonename _hititem _elementindex _faceindex _tracestart _traceend) (`GameplayStatics.BreakHitResult` _outhit))
  (bind _outhit_2 (`KismetSystemLibrary.LineTraceSingle` (`SceneComponent.GetSocketLocation` (`self.SK_Weapon_Mesh`) "Muzzle") (`KismetMathLibrary.SelectVector` (+ _location (* _returnvalue_2 10.0)) _traceend _returnvalue_3) "TraceTypeQuery1" false (`|MakeArray` (`self.PlayerRef`) :!type "Actor Object Reference") (select `bool` (`local.DrawDebug`) :`true` "ForOneFrame" :!type "EDrawDebugTrace Enum") true (struct :`R` 0.037764 :`G` 1.0 :`A` 1.0) (struct :`R` 0.008418 :`B` 1.0 :`A` 1.0)))
  (return _outhit_2))

(fn `UserConstructionScript`
  (`SkeletalMeshComponent.SetSkeletalMeshAsset` (`self.SK_Weapon_Mesh`) (`self.Mesh`)))