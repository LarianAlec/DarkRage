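; BP_ArenaVolume is a trigger volume that starts an arena encounter when the player character enters its box.
; On overlap it makes the HUD's arena counter widget visible, then tells the game mode to show markers above enemies and play arena music.
; A boolean set at the end makes it fire only once, provided the HUD counter widget was valid.
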(event `self.Box.OnComponentBeginOverlap`
  (params (OverlappedComponent :type "PrimitiveComponent Object Reference") (OtherActor :type "Actor Object Reference") (OtherComp :type "PrimitiveComponent Object Reference") (OtherBodyIndex :type Integer) (bFromSweep :type Boolean) (SweepResult :type "HitResult Structure (by ref)"))
  (if (not (`self.ArenaVolumeWasTriggered`))
    ;[1 1 1] Show Arena Counter in HUD
    (cast `/Game/DarkRage/Core/Characters/DarkRageCharacter/BP_DarkRageCharacter_Actual` OtherActor)
    (bind _asbp_dark_rage_hud (cast `/Game/DarkRage/Core/Blueprints/HUD/BP_DarkRage_HUD` (`PlayerController.GetHUD` (`GameplayStatics.GetPlayerController` 0))))
    (bind _wbp_arenacounter (`/Game/DarkRage/Core/Blueprints/HUD/BP_DarkRage_HUD.WBP_ArenaCounter` _asbp_dark_rage_hud)
      (:`then`
        (`Widget.SetVisibility` _wbp_arenacounter "Visible")
        ;[1 1 1] Show arena marker above enemy
        (bind _asgm_dark_rage_character_actual (cast `/Game/DarkRage/Core/Blueprints/GameModes/GM_DarkRageCharacter_Actual` (`GameplayStatics.GetGameMode`)))
        (`/Game/DarkRage/Core/Blueprints/GameModes/GM_DarkRageCharacter_Actual.ShowArenaMarkerAboveEnemy` _asgm_dark_rage_character_actual)
        ;[1 1 1] Play Arena Music
        (`/Game/DarkRage/Core/Blueprints/GameModes/GM_DarkRageCharacter_Actual.PlayArenaMusic` _asgm_dark_rage_character_actual)
        (set `self.ArenaVolumeWasTriggered` true))
      (:`else`))))

(fn `UserConstructionScript`)