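; Actor component that drops random loot around its owning AI character or enemy when it dies.
; It hooks the death event of the damage system on BP_AICharacter owners, or the died event on BP_Enemy owners.
; On death it rolls a drop chance and a random item count.
; Each item's class comes from a cumulative weighted pick over the ResorcesTable map, then spawns at a random point in a box around the owner.
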(event `self.ReceiveBeginPlay`
  (bind _returnvalue (`self.GetOwner`))
  (bind _asbp_aicharacter (cast `/Game/DarkRage/Core/AI/Character/BP_AICharacter` _returnvalue)
    (:`then`
      (add `/Game/DarkRage/Core/Blueprints/DamageSystem/BPC_DRDamageSystem.OnDeath` (`Actor.GetComponentByClass` _asbp_aicharacter "/Game/DarkRage/Core/Blueprints/DamageSystem/BPC_DRDamageSystem.BPC_DRDamageSystem_C") (delegate `DropLoot`)))
    (:`CastFailed`
      (bind _asbp_enemy (cast `/Game/AI_Characters/AI_Enemy_Base/BP_Enemy` _returnvalue))
      (add `/Game/AI_Characters/AI_Enemy_Base/BP_Enemy.OnDied` _asbp_enemy (delegate `DropLoot`)))))

(event `DropLoot`
  ;[1 1 1] Chance of Drop
  (if (<= (`KismetMathLibrary.RandomFloatInRange` 0.0 100.0) (`self.ChanceOfDrop`))
    ;[1 1 1] How many items drop?
    (bind _output_get (set `self.ItemsSpawnAmount` (`KismetMathLibrary.RandomIntegerInRange` (`self.MinItemsSpawnAmount`) (`self.MaxItemsSpawnAmount`))))
    (for _ (range 1 (+ _output_get 1))
      (`self.SpawnActualItem`))))

(event `SpawnActualItem`
  ;[1 1 1] Spawn actual item
  (bind _sum (`self.CalculateSum`))
  (set `self.Sum` _sum)
  (bind _loot (`self.ChooseLoot`))
  (`|SpawnActorFromClass` _loot (`KismetMathLibrary.MakeTransform` (`KismetMathLibrary.RandomPointInBoundingBox` (`Actor.K2_GetActorLocation` (`self.GetOwner`)) (100.0 100.0 20.0))) "Undefined" "MultiplyWithRoot" null null))

(fn `CalculateSum`
  (returns (Sum :type "Float (double-precision)"))
  (locals (RunningTotal :type "Float (double-precision)"))
  (bind _values (`BlueprintMapLibrary.Map_Values` (`self.ResorcesTable`)))
  (for _array_element _values
    (set `local.RunningTotal` (+ (`local.RunningTotal`) _array_element)))
  (return (`local.RunningTotal`)))

(fn `ChooseLoot`
  (returns (Loot :type "Actor Class Reference"))
  (locals (RandomValue :type "Float (double-precision)" :default 0.0))
  (set `local.RandomValue` (`KismetMathLibrary.RandomFloatInRange` 0.0 (`self.Sum`)))
  (bind _keys (`BlueprintMapLibrary.Map_Keys` (`self.ResorcesTable`)))
  (for _array_element _keys
    (bind _value (`BlueprintMapLibrary.Map_Find` (`self.ResorcesTable`) _array_element))
    (if (<= (`local.RandomValue`) _value)
      (return _array_element)
      (else
        (set `local.RandomValue` (- (`local.RandomValue`) _value))))))