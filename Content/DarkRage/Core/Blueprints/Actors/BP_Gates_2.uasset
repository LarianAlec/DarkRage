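; BP_Gates_2 is an arena gate that opens once all tagged arena enemies are dead.
; On BeginPlay it counts actors tagged ArenaEnemy and binds to the death event of each one's BPC_ArenaCounterComponent.
; When the count reaches zero, after a short delay the DoorRotator timeline moves the root along Z, despite its name.
; It also tells the game mode to show the gates-open HUD text and play calm ambient audio.
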(event `self.ReceiveBeginPlay`
  (`|ExecutionSequence`
    (:`then_0`
      (bind _outactors (`GameplayStatics.GetAllActorsWithTag` "ArenaEnemy"))
      (set `self.EnemiesCount` (`KismetArrayLibrary.Array_Length` _outactors))
      (for _array_element _outactors
        (bind _returnvalue (`self.FindComponentByTag` _array_element "/Game/DarkRage/Core/Blueprints/Components/BPC_ArenaCounterComponent.BPC_ArenaCounterComponent_C" "ArenaCounterComponent"))
        (`/Engine/EditorBlueprintResources/StandardMacros.IsValid` _returnvalue
          (:`Is Valid`
            (add `/Game/DarkRage/Core/Blueprints/Components/BPC_ArenaCounterComponent.OnDeath` _returnvalue (delegate `CheckEnemyCount`))))))))

(event `CheckEnemyCount`
  (bind _result (`/Engine/EditorBlueprintResources/StandardMacros.DecrementInt` (`self.EnemiesCount`))
    (:`  `
      (if (== _result 0)
        (`KismetSystemLibrary.Delay` 1.0)
        (`self.OpenGate`)
        ;[1 1 1] Show in HUD OpenGates_TextBlock
        (bind _asgm_dark_rage_character_actual (cast `/Game/DarkRage/Core/Blueprints/GameModes/GM_DarkRageCharacter_Actual` (`GameplayStatics.GetGameMode`)))
        (`/Game/DarkRage/Core/Blueprints/GameModes/GM_DarkRageCharacter_Actual.ShowTextBlockInHUD_OpenGates` _asgm_dark_rage_character_actual)
        (`/Game/DarkRage/Core/Blueprints/GameModes/GM_DarkRageCharacter_Actual.PlayCalmAmbient` _asgm_dark_rage_character_actual)))))

(event `OpenGate`
  (if (not (`self.IsOpened`))
    (bind (_direction _zlocation) (`Timeline|DoorRotator` :!via `PlayFromStart`)
      (:`Update`
        (`SceneComponent.K2_SetRelativeLocation` (`self.Root`) (`KismetMathLibrary.MakeVector` 0.0 0.0 _zlocation) false false))
      (:`Finished`
        (set `self.IsOpened` true)))))

(fn `UserConstructionScript`)