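; Base AI enemy character that delegates health, damage, healing and attack tokens to a DR damage system component and shows a health bar widget.
; Damage responses trigger a timed hit-reaction flag or a stagger montage that freezes the AI controller before it resumes attacking.
; Attacks reserve tokens from the target, tracked per target and returned on attack end or death.
; Death ragdolls the mesh and stops AI logic.
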(event `self.ReceiveBeginPlay`
  (bind _bpc_drdamagesystem (`self.BPC_DRDamageSystem`))
  ;[0.01945 1 0.9502] BeginPlay
  (bind _asaic_character (cast `/Game/DarkRage/Core/AI/Character/AIC_Character` (`AIBlueprintHelperLibrary.GetAIController` self)))
  (set `self.AIC Character` _asaic_character)
  (bind _returnvalue (`|CreateWidget` "/Game/DarkRage/Core/Blueprints/DamageSystem/WBP_DRHealthBar.WBP_DRHealthBar_C" null self))
  (`WidgetComponent.SetWidget` (`self.Widget`) _returnvalue)
  (add `/Game/DarkRage/Core/Blueprints/DamageSystem/BPC_DRDamageSystem.OnDeath` _bpc_drdamagesystem (`|CreateDelegate` :!event `Die`))
  (add `/Game/DarkRage/Core/Blueprints/DamageSystem/BPC_DRDamageSystem.OnDamageResponse` _bpc_drdamagesystem (`|CreateDelegate` :!event `HitResponse`)))

(event `self.ReceiveAnyDamage`
  (params (Damage :type "Float (single-precision)") (DamageType :type "DamageType Object Reference") (InstigatedBy :type "Controller Object Reference") (DamageCauser :type "Actor Object Reference"))
  ;[1 0.01813 0] Recieving AnyDamage
  (`/Game/DarkRage/Core/Blueprints/DamageSystem/BPC_DRDamageSystem.TakeDamage` (`self.BPC_DRDamageSystem`) (make `/Game/DarkRage/Core/Blueprints/DamageSystem/S_DRDamageInfo` Damage "NewEnumerator2" "NewEnumerator1")))

(event `Die`
  (bind _mesh (`self.Mesh`))
  ;[1 0.01813 0] Death
  (`PrimitiveComponent.SetSimulatePhysics` _mesh true)
  (`PrimitiveComponent.SetCollisionEnabled` _mesh "QueryAndPhysics")
  (`PrimitiveComponent.SetCollisionEnabled` (`self.CapsuleComponent`) "NoCollision")
  (`BrainComponent.StopLogic` (`AIController.BrainComponent` (`self.AIC Character`)) "")
  (`/Game/DarkRage/Core/AI/Character/AIC_Character.SetStateAsDead` (`self.AIC Character`))
  (bind _keys (`BlueprintMapLibrary.Map_Keys` (`self.ReservedAttackTokens`)))
  (for _array_element _keys
    (message `/Game/DarkRage/Core/Blueprints/DamageSystem/BPI_DRDamageSystem.ReturnAttackToken` _array_element (`BlueprintMapLibrary.Map_Find` (`self.ReservedAttackTokens`) _array_element))))

(event `HitResponse`
  (params (DamageResponse :type "/Game/DarkRage/Core/Blueprints/DamageSystem/E_DRDamageResponse Enum" :default "NewEnumerator0"))
  ;[1 0.01813 0] HitResponse
  (switch `/Game/DarkRage/Core/Blueprints/DamageSystem/E_DRDamageResponse` DamageResponse
    (:`NewEnumerator1`
      ;;[1 1 1] Switch
      (set `self.IsGotHit` true)
      (`KismetSystemLibrary.RetriggerableDelay` (`self.AdditiveHitReactionDuration`))
      (set `self.IsGotHit` false))
    (:`NewEnumerator2`
      (`MovementComponent.StopMovementImmediately` (`self.CharacterMovement`))
      (`/Game/DarkRage/Core/AI/Character/AIC_Character.SetStateAsFrozen` (`self.AIC Character`))
      (`|PlayMontage` (`self.Mesh`) (`self.StaggerAnimMontage`)
        (:`OnCompleted`
          _)
        (:`OnInterrupted`
          _))
      (`/Game/DarkRage/Core/AI/Character/AIC_Character.SetStateAsAttacking` (`self.AIC Character`) null true))))

(event `/Game/DarkRage/Core/Blueprints/DamageSystem/BPI_DRDamageSystem.ReturnAttackToken`
  (params (Amount :type Integer))
  ;[1 0.01813 0] Return Attack Token
  (`/Game/DarkRage/Core/Blueprints/DamageSystem/BPC_DRDamageSystem.ReturnAttackToken` (`self.BPC_DRDamageSystem`) Amount))

(event `/Game/DarkRage/Core/AI/Character/Interfaces/BPI_AICharacter.StoreAttackTokens`
  (params (AttackTarget :type "Actor Object Reference") (Amount :type Integer))
  (bind (_value _returnvalue) (`BlueprintMapLibrary.Map_Find` (`self.ReservedAttackTokens`) AttackTarget))
  ;[1 0.01813 0] StoreAttackTokens
  (`BlueprintMapLibrary.Map_Add` (`self.ReservedAttackTokens`) AttackTarget (`KismetMathLibrary.SelectInt` (+ Amount _value) Amount _returnvalue)))

(event `/Game/DarkRage/Core/AI/Character/Interfaces/BPI_AICharacter.Attack`
  (params (AttackTarget :type "Actor Object Reference"))
  ;[1 0.01813 0] Attack
  (set `self.Attacking` true))

(event `/Game/DarkRage/Core/AI/Character/Interfaces/BPI_AICharacter.AttackEnd`
  (params (AttackTarget :type "Actor Object Reference"))
  (bind _tokensusedincurrentattack (`self.TokensUsedInCurrentAttack`))
  ;[1 0.01813 0] Attack End
  (message `/Game/DarkRage/Core/Blueprints/DamageSystem/BPI_DRDamageSystem.ReturnAttackToken` AttackTarget _tokensusedincurrentattack)
  (`/Game/DarkRage/Core/AI/Character/Interfaces/BPI_AICharacter.StoreAttackTokens` AttackTarget (* _tokensusedincurrentattack -1))
  (`self.OnAttackEnd`)
  (set `self.Attacking` false))

(fn `AttackStart`
  (params (AttackTarget :type "Actor Object Reference") (TokensNeeded :type Integer))
  (returns (Success :type Boolean))
  (bind _success (message `/Game/DarkRage/Core/Blueprints/DamageSystem/BPI_DRDamageSystem.ReserveAttackToken` AttackTarget TokensNeeded))
  (if _success
    (`/Game/DarkRage/Core/AI/Character/Interfaces/BPI_AICharacter.StoreAttackTokens` AttackTarget TokensNeeded)
    (set `self.TokensUsedInCurrentAttack` TokensNeeded)
    (return true)
    (else
      (return false))))

(fn `GetCurrentHelath`
  (returns (Health :type "Float (double-precision)"))
  (return (`/Game/DarkRage/Core/Blueprints/DamageSystem/BPC_DRDamageSystem.Health` (`self.BPC_DRDamageSystem`))))

(fn `GetIdealRange`
  (returns (AttackRadius :type "Float (double-precision)") (DefendRadius :type "Float (double-precision)"))
  (return 150.0 400.0))

(fn `GetMaxHealth`
  (returns (MaxHealth :type "Float (double-precision)"))
  (return (`/Game/DarkRage/Core/Blueprints/DamageSystem/BPC_DRDamageSystem.MaxHealth` (`self.BPC_DRDamageSystem`))))

(fn `GetPatrolPathway`
  (returns (PatrolPathway :type "/Game/DarkRage/Core/Blueprints/Actors/BP_PatrolPathway Object Reference"))
  (return (`self.PatrolPathway`)))

(fn `Heal`
  (params (Amount :type "Float (double-precision)"))
  (returns (NewHealth :type "Float (double-precision)"))
  (bind _newhealth (`/Game/DarkRage/Core/Blueprints/DamageSystem/BPC_DRDamageSystem.Heal` (`self.BPC_DRDamageSystem`) Amount))
  (return _newhealth))

(fn `IsDead`
  (returns (IsDead :type Boolean))
  (return (`/Game/DarkRage/Core/Blueprints/DamageSystem/BPC_DRDamageSystem.IsDead` (`self.BPC_DRDamageSystem`))))

(fn `ReserveAttackToken`
  (params (Amount :type Integer))
  (returns (Success :type Boolean))
  (bind _success (`/Game/DarkRage/Core/Blueprints/DamageSystem/BPC_DRDamageSystem.ReserveAttackToken` (`self.BPC_DRDamageSystem`) Amount))
  (return _success))

(fn `SetMovementSpeed`
  (params (NewSpeed :type "/Game/DarkRage/Core/AI/Character/Enums/E_MovementAISpeed Enum" :default "NewEnumerator0"))
  (returns (CurrentSpeed :type "Float (double-precision)"))
  (bind _output_get (set `CharacterMovementComponent.MaxWalkSpeed` (select `/Game/DarkRage/Core/AI/Character/Enums/E_MovementAISpeed` NewSpeed :`NewEnumerator1` 125.0 :`NewEnumerator4` 215.0 :`NewEnumerator2` 300.0 :`NewEnumerator3` 550.0 :!type "Float (single-precision)") (`self.CharacterMovement`)))
  (return _output_get))

(fn `TakeDamage`
  (params (DamageInput :type "/Game/DarkRage/Core/Blueprints/DamageSystem/S_DRDamageInfo Structure"))
  (returns (WasDamaged :type Boolean))
  (bind _wasdamaged (`/Game/DarkRage/Core/Blueprints/DamageSystem/BPC_DRDamageSystem.TakeDamage` (`self.BPC_DRDamageSystem`) DamageInput))
  (return _wasdamaged))

(fn `UserConstructionScript`)