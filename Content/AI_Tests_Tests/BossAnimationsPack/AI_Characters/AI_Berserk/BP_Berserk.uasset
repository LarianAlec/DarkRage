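; Berserker AI enemy that fights with an axe, spawned and destroyed on equip/unequip montage notifies, and can drop random loot.
; Point damage drives BPCEnemy health, with double headshot damage and a camera-facing health bar shown briefly on hit.
; The first hit reaching half health triggers a one-time burst: current health halves, a power montage grants immunity, then damage taken increases.
; HealthMult scales incoming damage, also blocking it during equip.
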(event `self.ReceiveTick`
  (params (DeltaSeconds :type "Float (single-precision)"))
  (bind _w_healthbar (`self.W_HealthBar`))
  ;[1 1 1] event tick on updata widjet rotation
  (`parent.ReceiveTick` DeltaSeconds)
  (`SceneComponent.K2_SetWorldRotation` _w_healthbar (`KismetMathLibrary.FindLookAtRotation` (`SceneComponent.K2_GetComponentLocation` _w_healthbar) (`SceneComponent.K2_GetComponentLocation` (`PlayerCameraManager.TransformComponent` (`GameplayStatics.GetPlayerCameraManager` 0)))) false false))

(event `self.ReceiveBeginPlay`
  (bind _pawnhealth (`self.PawnHealth`))
  (bind _bpc_enemy (`self.BPC_Enemy`))
  (`parent.ReceiveBeginPlay`)
  (set `self.DeathMontage` "/Game/AI_Tests_Tests/BossAnimationsPack/AI_Characters/AI_Berserk/Animation_Berserk/EssentialGreatSwordAnimationPack/Animation/Sequence/Hurt_Die/1H-B_Die_01_Seq_Montage.1H-B_Die_01_Seq_Montage")
  (set `/Game/AI_Tests_Tests/BossAnimationsPack/AI_Characters/AI_Enemy_Base/BPC_Enemy.Health` _pawnhealth _bpc_enemy)
  (set `/Game/AI_Tests_Tests/BossAnimationsPack/AI_Characters/AI_Enemy_Base/BPC_Enemy.MaxHealth` _pawnhealth _bpc_enemy)
  (bind _returnvalue (`|CreateWidget` "/Game/AI_Tests_Tests/BossAnimationsPack/AI_Characters/AI_Enemy_Base/Bar_for_enemy/W_HealthBarAI.W_HealthBarAI_C" null self))
  (`WidgetComponent.SetWidget` (`self.W_HealthBar`) _returnvalue)
  (add `self.OnTakePointDamage` (delegate `OnTakePointDamage_Event`)))

(event `OnTakePointDamage_Event`
  (params (DamagedActor :type "Actor Object Reference") (Damage :type "Float (single-precision)") (InstigatedBy :type "Controller Object Reference") (HitLocation :type "Vector Structure") (FHitComponent :type "PrimitiveComponent Object Reference") (BoneName :type Name) (ShotFromDirection :type "Vector Structure") (DamageType :type "DamageType Object Reference") (DamageCauser :type "Actor Object Reference"))
  (bind _bpc_enemy (`self.BPC_Enemy`))
  (bind _bpc_enemy_2 (`self.BPC_Enemy`))
  (bind _w_healthbar (`self.W_HealthBar`))
  (bind _bpc_enemy_3 (`self.BPC_Enemy`))
  (bind _returnvalue (- (`/Game/AI_Tests_Tests/BossAnimationsPack/AI_Characters/AI_Enemy_Base/BPC_Enemy.Health` _bpc_enemy_3) (* (* Damage (`KismetMathLibrary.SelectFloat` 2.0 1.0 (== BoneName "head"))) (`self.HealthMult`))))
  ;[1 0.05098 0] Apply Damage And Death via c++
  ;[1 1 1] Widjet
  (`|ExecutionSequence`
    (:`then_0`
      (`SceneComponent.SetHiddenInGame` _w_healthbar false false)
      (`KismetSystemLibrary.Delay` 5.0)
      (`SceneComponent.SetHiddenInGame` _w_healthbar true false))
    (:`then_1`
      (`AISense_Damage.ReportDamageEvent` DamagedActor InstigatedBy Damage ShotFromDirection)
      (set `self.Hit Location` HitLocation)
      (set `/Game/AI_Tests_Tests/BossAnimationsPack/AI_Characters/AI_Enemy_Base/BPC_Enemy.BurstBerserk` (>= (/ (`/Game/AI_Tests_Tests/BossAnimationsPack/AI_Characters/AI_Enemy_Base/BPC_Enemy.MaxHealth` _bpc_enemy_3) 2.0) _returnvalue) _bpc_enemy)
      (if (`/Game/AI_Tests_Tests/BossAnimationsPack/AI_Characters/AI_Enemy_Base/BPC_Enemy.BurstBerserk` _bpc_enemy)
        (if (`/Game/AI_Tests_Tests/BossAnimationsPack/AI_Characters/AI_Enemy_Base/BPC_Enemy.BurstKeyBerserk` _bpc_enemy)
          (set `/Game/AI_Tests_Tests/BossAnimationsPack/AI_Characters/AI_Enemy_Base/BPC_Enemy.BurstKeyBerserk` false _bpc_enemy_2)
          (set `self.HealthMult` 0.0)
          (set `/Game/AI_Tests_Tests/BossAnimationsPack/AI_Characters/AI_Enemy_Base/BPC_Enemy.Health` (/ (`/Game/AI_Tests_Tests/BossAnimationsPack/AI_Characters/AI_Enemy_Base/BPC_Enemy.Health` _bpc_enemy_2) 2.0) _bpc_enemy_2)
          (`|PlayMontage` (`self.Mesh`) "/Game/AI_Tests_Tests/BossAnimationsPack/AI_Characters/AI_Berserk/Animation_Berserk/EssentialGreatSwordAnimationPack/Animation/Sequence/Power/1H_Power_01_Seq_Montage.1H_Power_01_Seq_Montage"
            (:`OnCompleted`
              _)
            (:`OnInterrupted`
              _))
          (set `self.HealthMult` 1.5)
          (else
            (bind _output_get (set `/Game/AI_Tests_Tests/BossAnimationsPack/AI_Characters/AI_Enemy_Base/BPC_Enemy.Health` _returnvalue (`self.BPC_Enemy`) :!label _label))))
        (else
          (goto _label)))
      (if (<= _output_get 0.0)
        (`self.Died`)))))

(event `Died`
  ;[1 1 1] Death
  (`SceneComponent.SetHiddenInGame` (`self.W_HealthBar`) true false)
  (`self.AI_Death` null))

(event `/Game/AI_Tests_Tests/BossAnimationsPack/AI_Characters/AI_Enemy_Base/BPI_Enemy.EquipWeapon`
  ;[1 1 1] Equip Axe
  (set `self.HealthMult` 0.0)
  (bind _notifyname (`|PlayMontage` (`self.Mesh`) "/Game/AI_Tests_Tests/BossAnimationsPack/AI_Characters/AI_Berserk/Animation_Berserk/EssentialGreatSwordAnimationPack/Animation/Sequence/Equip/1H-B_Equip_02_Seq_Montage.1H-B_Equip_02_Seq_Montage")
    (:`OnCompleted`
      (`self.OnWealdAxe`)
      (set `self.HealthMult` 1.0)
      (set `self.IsWeildingWeapon` true))
    (:`OnNotifyBegin`
      (switch `name` _notifyname
        (:`HoldAxe`
          (bind _returnvalue (`|SpawnActorFromClass` "/Game/AI_Tests_Tests/BossAnimationsPack/AI_Characters/Weapon_AI/Berserk/BB_Weapon_Axe_Berserk.BB_Weapon_Axe_Berserk_C" (`self.GetTransform`) "Undefined" "MultiplyWithRoot" null null))
          (bind _output_get (set `self.WeaponActor` _returnvalue))
          (`self.K2_AttachToComponent` _output_get (`self.Mesh`) "hand_r_Axe" "SnapToTarget" "SnapToTarget" "SnapToTarget" true))))))

(event `/Game/AI_Tests_Tests/BossAnimationsPack/AI_Characters/AI_Enemy_Base/BPI_Enemy.UnequipWeapon`
  (bind _weaponactor (`self.WeaponActor`))
  ;[1 1 1] Unequip Axe
  (set `self.IsWeildingWeapon` false)
  (bind _notifyname (`|PlayMontage` (`self.Mesh`) "/Game/AI_Tests_Tests/BossAnimationsPack/AI_Characters/AI_Berserk/Animation_Berserk/EssentialGreatSwordAnimationPack/Animation/Sequence/Equip/1H-B_Unequip_01_Seq_Montage.1H-B_Unequip_01_Seq_Montage")
    (:`then`
      (`self.OnSheathAxe`))
    (:`OnNotifyBegin`
      (switch `name` _notifyname
        (:`DropAxe`
          (if (`KismetSystemLibrary.IsValid` _weaponactor)
            (`self.K2_DestroyActor` _weaponactor)))))))

(event `/Game/UEGameCode/Core/Interfaces/BPI_Damage.ReceiveDamage`
  (params (Damage :type "Float (double-precision)") (ImpactLocation :type "Vector Structure") (HitBoneName :type Name))
  ;[0.3333 0.02491 0 1 30] Apply Damage and Death (old)
)

(event `DropLoot`
  (bind _returnvalue (`SceneComponent.K2_GetComponentLocation` (`self.Mesh`)))
  ;[0 0.01693 0.4948] DropLoot
  (bind _outhit (`KismetSystemLibrary.LineTraceSingle` _returnvalue (+ _returnvalue (`KismetMathLibrary.MakeVector` 0.0 0.0 (`KismetMathLibrary.RandomFloatInRange` 0.0 200.0))) "TraceTypeQuery1"))
  (`KismetSystemLibrary.PrintString` "spawn loot")
  (`|SpawnActorFromClass` (select `int` (`KismetMathLibrary.RandomInteger` 3) :`0` "/Game/AI_Tests_Tests/BossAnimationsPack/AI_Characters/AI_Enemy_Base/LootFromEnemy/HealthLoot.HealthLoot_C" :`1` "/Game/AI_Tests_Tests/BossAnimationsPack/AI_Characters/AI_Enemy_Base/LootFromEnemy/AmmoLoot1.AmmoLoot1_C" :`2` "/Game/AI_Tests_Tests/BossAnimationsPack/AI_Characters/AI_Enemy_Base/LootFromEnemy/AmmoLoot2.AmmoLoot2_C" :`3` "/Game/AI_Tests_Tests/BossAnimationsPack/AI_Characters/AI_Enemy_Base/LootFromEnemy/AmmoLoot3.AmmoLoot3_C" :!type "Actor Class Reference") (`KismetMathLibrary.MakeTransform` (+ (`.Location` (`GameplayStatics.BreakHitResult` _outhit)) (`KismetMathLibrary.MakeVector` (`KismetMathLibrary.RandomFloatInRange` 0.0 200.0) (`KismetMathLibrary.RandomFloatInRange` 0.0 200.0))) (`KismetMathLibrary.MakeRotator` 0.0 0.0 (`KismetMathLibrary.RandomFloatInRange` 0.0 360.0))) "Undefined" "MultiplyWithRoot" null null))

(fn `Get CurrentHealth`
  (returns (Health :type "Float (double-precision)"))
  (return (`/Game/AI_Tests_Tests/BossAnimationsPack/AI_Characters/AI_Enemy_Base/BPC_Enemy.Health` (`self.BPC_Enemy`))))

(fn `Get MaxHealth`
  (returns (MaxHealth :type "Float (double-precision)"))
  (return (`/Game/AI_Tests_Tests/BossAnimationsPack/AI_Characters/AI_Enemy_Base/BPC_Enemy.MaxHealth` (`self.BPC_Enemy`))))

(fn `UserConstructionScript`
  (`parent.UserConstructionScript`))