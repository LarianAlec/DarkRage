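; Bear boss enemy "Отец", with a health/armor bar shown on aggro and removed on death.
; Point damage drains armor before health and doubles on headshots; dropping to two-thirds and one-third health advances the stage and refills armor.
; Montage notifies spawn or destroy hand-socketed spears, including a dual-spear second-stage draw, with HealthMult zeroed during equips for invulnerability.
; A timeline lerps dash attacks, and a landing callback halts jump-attack movement.
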(event `self.ReceiveBeginPlay`
  (bind _bpc_enemy (`self.BPC_Enemy`))
  (bind _pawn_health (`self.Pawn Health`))
  (bind _pawn_armor (`self.Pawn Armor`))
  (`parent.ReceiveBeginPlay`)
  (set `/Game/AI_Tests_Tests/BossAnimationsPack/AI_Characters/AI_Enemy_Base/BPC_Enemy.EnemyName` "Отец" (`self.BPC_Enemy`))
  (set `self.DeathMontage` "/Game/AI_Tests_Tests/BossAnimationsPack/AI_Characters/AI_Bear_Boss/Animation/Frank_RPG_Spear/Animations/Mannequin/Frank_RPG_Spear_Die03_Montage.Frank_RPG_Spear_Die03_Montage")
  (set `/Game/AI_Tests_Tests/BossAnimationsPack/AI_Characters/AI_Enemy_Base/BPC_Enemy.Health` _pawn_health _bpc_enemy)
  (set `/Game/AI_Tests_Tests/BossAnimationsPack/AI_Characters/AI_Enemy_Base/BPC_Enemy.MaxHealth` _pawn_health _bpc_enemy)
  (set `/Game/AI_Tests_Tests/BossAnimationsPack/AI_Characters/AI_Enemy_Base/BPC_Enemy.Armor` _pawn_armor _bpc_enemy)
  (set `/Game/AI_Tests_Tests/BossAnimationsPack/AI_Characters/AI_Enemy_Base/BPC_Enemy.MaxArmor` _pawn_armor _bpc_enemy)
  (bind _returnvalue (`|CreateWidget` "/Game/AI_Tests_Tests/BossAnimationsPack/AI_Characters/AI_Enemy_Base/Bar_for_Boss/BossWithArmo/W_HealthBarAI_testArmor.W_HealthBarAI_testArmor_C" null self))
  (set `self.BossBar` _returnvalue)
  (add `self.OnTakePointDamage` (delegate `OnTakePointDamage_Event`)))

(event `self.ReceiveTick`
  (params (DeltaSeconds :type "Float (single-precision)"))
  (`parent.ReceiveTick` DeltaSeconds)
  (`self.UpdateStage`)
  (if (`self.BarIsUsed?`)
    _
    (elif (`self.AgroState`)
      (`UserWidget.AddToViewport` (`self.BossBar`) 0)
      (set `self.BarIsUsed?` true))))

(event `OnTakePointDamage_Event`
  (params (DamagedActor :type "Actor Object Reference") (Damage :type "Float (single-precision)") (InstigatedBy :type "Controller Object Reference") (HitLocation :type "Vector Structure") (FHitComponent :type "PrimitiveComponent Object Reference") (BoneName :type Name) (ShotFromDirection :type "Vector Structure") (DamageType :type "DamageType Object Reference") (DamageCauser :type "Actor Object Reference"))
  (bind _bpc_enemy (`self.BPC_Enemy`))
  (bind _bpc_enemy_2 (`self.BPC_Enemy`))
  (bind _health (`/Game/AI_Tests_Tests/BossAnimationsPack/AI_Characters/AI_Enemy_Base/BPC_Enemy.Health` _bpc_enemy_2))
  (bind _armor (`/Game/AI_Tests_Tests/BossAnimationsPack/AI_Characters/AI_Enemy_Base/BPC_Enemy.Armor` _bpc_enemy_2))
  ;[1 1 1] TakeDamage
  (set `self.Hit Location` HitLocation)
  (`AISense_Damage.ReportDamageEvent` DamagedActor InstigatedBy 1.0 ShotFromDirection)
  (set `self.ReciveDamage` (* (`self.HealthMult`) (* Damage (`KismetMathLibrary.SelectFloat` 2.0 1.0 (== BoneName "head")))))
  (if (== _armor 0.0)
    (bind _output_get (set `/Game/AI_Tests_Tests/BossAnimationsPack/AI_Characters/AI_Enemy_Base/BPC_Enemy.Health` (- _health (`self.ReciveDamage`)) (`self.BPC_Enemy`)))
    (if (<= _output_get 0.0)
      (`self.Death`))
    (elif (> (`self.ReciveDamage`) _armor)
      (bind _output_get_2 (set `/Game/AI_Tests_Tests/BossAnimationsPack/AI_Characters/AI_Enemy_Base/BPC_Enemy.Health` (- (+ _armor _health) (`self.ReciveDamage`)) _bpc_enemy))
      (set `/Game/AI_Tests_Tests/BossAnimationsPack/AI_Characters/AI_Enemy_Base/BPC_Enemy.Armor` 0.0 _bpc_enemy)
      (if (<= _output_get_2 0.0)
        (`self.Death`))
      (else
        (set `/Game/AI_Tests_Tests/BossAnimationsPack/AI_Characters/AI_Enemy_Base/BPC_Enemy.Armor` (- _armor (`self.ReciveDamage`)) (`self.BPC_Enemy`))))))

(event `Death`
  ;[1 1 1] Death
  (bind _bossbar (`self.BossBar`)
    (:`then`
      (`Widget.RemoveFromParent` _bossbar))
    (:`else`
      _))
  (bind _weaponactor_2h (`self.WeaponActor_2H`)
    (:`then`
      (`self.AI_Death` _weaponactor_2h))
    (:`else`
      (`self.AI_Death` null))))

(event `UpdateStage`
  (bind _stage (`self.Stage`))
  (bind _bpc_enemy (`self.BPC_Enemy`))
  (bind _health (`/Game/AI_Tests_Tests/BossAnimationsPack/AI_Characters/AI_Enemy_Base/BPC_Enemy.Health` _bpc_enemy))
  (bind _maxhealth (`/Game/AI_Tests_Tests/BossAnimationsPack/AI_Characters/AI_Enemy_Base/BPC_Enemy.MaxHealth` _bpc_enemy))
  ;[1 1 1] UpdateStage
  (if (<= _health (/ _maxhealth 3.0))
    (if (not (== _stage "Third"))
      (set `self.Stage` "Third")
      (set `/Game/AI_Tests_Tests/BossAnimationsPack/AI_Characters/AI_Enemy_Base/BPC_Enemy.Armor` (`self.Pawn Armor`) (`self.BPC_Enemy`) :!label _label))
    (elif (<= _health (* (/ _maxhealth 3.0) 2.0))
      (if (not (== _stage "Second"))
        (set `self.Stage` "Second")
        (goto _label)))))

(event `/Game/AI_Tests_Tests/BossAnimationsPack/AI_Characters/AI_Enemy_Base/BPI_Enemy.EquipWeapon`
  ;[1 1 1] EquipWeapon
  (set `self.IsWeildingWeapon` true)
  (set `self.HealthMult` 0.0)
  (bind _notifyname (`|PlayMontage` (`self.Mesh`) "/Game/AI_Tests_Tests/BossAnimationsPack/AI_Characters/AI_Bear_Boss/Animation/USED/OneSpearStage/Equip_Unequip/Frank_RPG_Spear_Equip_Montage.Frank_RPG_Spear_Equip_Montage")
    (:`OnCompleted`
      (set `self.HealthMult` 1.0)
      (`self.OnWealdAxe`))
    (:`OnNotifyBegin`
      (switch `name` _notifyname
        (:`Hold`
          (bind _returnvalue (`|SpawnActorFromClass` "/Game/AI_Tests_Tests/BossAnimationsPack/AI_Characters/Weapon_AI/Bear_Boss/BP_Bear_Spear.BP_Bear_Spear_C" (`self.GetTransform`) "Undefined" "MultiplyWithRoot" null null))
          (bind _output_get (set `self.WeaponActor` _returnvalue))
          (`self.K2_AttachToComponent` _output_get (`self.Mesh`) "hand_rSocket" "SnapToTarget" "SnapToTarget" "SnapToTarget" true))))))

(event `/Game/AI_Tests_Tests/BossAnimationsPack/AI_Characters/AI_Enemy_Base/BPI_Enemy.UnequipWeapon`
  (bind _weaponactor (`self.WeaponActor`))
  ;[1 1 1] Unequip Weapon
  (set `self.IsWeildingWeapon` false)
  (bind _notifyname (`|PlayMontage` (`self.Mesh`) "/Game/AI_Tests_Tests/BossAnimationsPack/AI_Characters/AI_Berserk/Animation_Berserk/EssentialGreatSwordAnimationPack/Animation/Sequence/Equip/1H-B_Unequip_01_Seq_Montage.1H-B_Unequip_01_Seq_Montage")
    (:`then`
      (`self.OnSheathAxe`))
    (:`OnNotifyBegin`
      (switch `name` _notifyname
        (:`DropAxe`
          (if (`KismetSystemLibrary.IsValid` _weaponactor)
            (`self.K2_DestroyActor` _weaponactor)))))))

(event `/Game/AI_Tests_Tests/BossAnimationsPack/AI_Characters/AI_Enemy_Base/BPI_Enemy.EquipWeaponBossStage Second`
  ;[1 1 1] Equip Weapon
  (set `self.HealthMult` 0.0)
  (bind _notifyname (`|PlayMontage` (`self.Mesh`) "/Game/AI_Tests_Tests/BossAnimationsPack/AI_Characters/AI_Bear_Boss/Animation/Frank_RPG_Dual/Animations/Mannequin_RootMotion/Frank_RPG_Dual_Draw_Montage.Frank_RPG_Dual_Draw_Montage" 0.5)
    (:`OnCompleted`
      (set `self.HealthMult` 1.0)
      (`self.OnWealdWeapon`))
    (:`OnNotifyBegin`
      (switch `name` _notifyname
        (:`Hold`
          (`self.WeaponActor`
            (:`then`
              _)
            (:`else`
              ;[1 1 1] first weapon
              (bind _returnvalue (`|SpawnActorFromClass` "/Game/AI_Tests_Tests/BossAnimationsPack/AI_Characters/Weapon_AI/Bear_Boss/BP_Bear_Spear.BP_Bear_Spear_C" (`self.GetTransform`) "Undefined" "MultiplyWithRoot" null null))
              (bind _output_get (set `self.WeaponActor` _returnvalue))
              (`self.K2_AttachToComponent` _output_get (`self.Mesh`) "hand_rSocket" "SnapToTarget" "SnapToTarget" "SnapToTarget" true)))
          (bind _returnvalue_2 (`|SpawnActorFromClass` "/Game/AI_Tests_Tests/BossAnimationsPack/AI_Characters/Weapon_AI/Bear_Boss/BP_Bear_Spear.BP_Bear_Spear_C" (`self.GetTransform`) "Undefined" "MultiplyWithRoot" null null))
          (bind _output_get_2 (set `self.WeaponActor_2H` _returnvalue_2))
          (`self.K2_AttachToComponent` _output_get_2 (`self.Mesh`) "hand_lSocket" "SnapToTarget" "SnapToTarget" "SnapToTarget" true)
          (set `self.IsWeildingWeapon` false)
          (set `self.IsWeildingWeapon2H` true))))))

(event `DashTimeLine`
  ;[1 1 1] DashAttackLine
  (set `self.StartLocation` (`self.K2_GetActorLocation`))
  (bind (_direction _longattack) (`Timeline|Timeline` :!via `PlayFromStart`)
    (:`Update`
      (`self.K2_SetActorLocation` (`KismetMathLibrary.VLerp` (`self.StartLocation`) (`self.EndLocation`) _longattack)))))

(event `for jump attack`
  ;[1 1 1] ForJump
  (add `self.LandedDelegate` (delegate `LandedDelegate_Event`)))

(event `LandedDelegate_Event` :!signature `self.LandedDelegate`
  (params (Hit :type "HitResult Structure (by ref)"))
  ;[1 1 1] ForJump
  (remove `self.LandedDelegate` (delegate `LandedDelegate_Event`))
  (`MovementComponent.StopMovementImmediately` (`self.CharacterMovement`)))

(fn `Get CurrentArmor`
  (returns (CurrentArmor :type "Float (double-precision)"))
  (return (`/Game/AI_Tests_Tests/BossAnimationsPack/AI_Characters/AI_Enemy_Base/BPC_Enemy.Armor` (`self.BPC_Enemy`))))

(fn `Get CurrentHealth`
  (returns (Health :type "Float (double-precision)"))
  (return (`/Game/AI_Tests_Tests/BossAnimationsPack/AI_Characters/AI_Enemy_Base/BPC_Enemy.Health` (`self.BPC_Enemy`))))

(fn `Get MaxArmor`
  (returns (MaxArmor :type "Float (double-precision)"))
  (return (`/Game/AI_Tests_Tests/BossAnimationsPack/AI_Characters/AI_Enemy_Base/BPC_Enemy.MaxArmor` (`self.BPC_Enemy`))))

(fn `Get MaxHealth`
  (returns (MaxHealth :type "Float (double-precision)"))
  (return (`/Game/AI_Tests_Tests/BossAnimationsPack/AI_Characters/AI_Enemy_Base/BPC_Enemy.MaxHealth` (`self.BPC_Enemy`))))

(fn `GetEnemyName`
  (returns (Name :type Text))
  (return (`/Game/AI_Tests_Tests/BossAnimationsPack/AI_Characters/AI_Enemy_Base/BPC_Enemy.EnemyName` (`self.BPC_Enemy`))))

(fn `UserConstructionScript`
  (`parent.UserConstructionScript`))