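; Legacy player controller for DarkRage that handles player-level input for pausing, the upgrades panel and restarting.
; On BeginPlay it adds the first-person Enhanced Input mapping context and caches the HUD base.
; The pause action creates the pause menu and pauses the game, while the unpause toggle branch is left disconnected.
; A hard-wired U key toggles the HUD's upgrades panel, and the restart action forwards to the controlled legacy character.
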(event `self.ReceiveBeginPlay`
  (`|ExecutionSequence`
    (:`then_0`
      ;[1 0.2059 0.2656 1 50] ENHANCED INPUT SYSTEM Add Input Mapping
      (bind _asbp_dark_rage_player_controller_legacy (cast `/Game/UEGameCode/Core/Blueprints/BP_DarkRagePlayerController_LEGACY` (`GameplayStatics.GetPlayerController` 0)))
      (bind _returnvalue (pcsubsystem `EnhancedInputLocalPlayerSubsystem` _asbp_dark_rage_player_controller_legacy))
      (`/Engine/EditorBlueprintResources/StandardMacros.IsValid` _returnvalue
        (:`Is Valid`
          (`EnhancedInputSubsystemInterface.AddMappingContext` _returnvalue "/Game/UEGameCode/Core/Input/IMC_FirstPersonPlayer.IMC_FirstPersonPlayer" 0 (struct)))))
    (:`then_1`
      (bind _asbp_hud_base (`/Game/UEGameCode/Core/MacroLibraries/BML_PlayerController.GET_BP_HUD_BASE` 10.0)
        (:`Success`
          (set `self.As BP HUD Base` _asbp_hud_base))))))

(event `EnhancedInput|/Game/DarkRage/Core/Input/Actions/IA_PauseMenu`
  (params (ActionValue :type Boolean) (ElapsedSeconds :type "Float (double-precision)") (TriggeredSeconds :type "Float (double-precision)") (InputAction :type "InputAction Object Reference" :default "/Game/DarkRage/Core/Input/Actions/IA_PauseMenu.IA_PauseMenu"))
  (:`Triggered`
    (set `self.IsGamePaused` true)
    (bind _returnvalue (`|CreateWidget` "/Game/UEGameCode/UI/WBP_PauseMenu.WBP_PauseMenu_C" (`GameplayStatics.GetPlayerController` 0)))
    (bind _output_get (set `self.PauseMenuWidget` _returnvalue))
    (`UserWidget.AddToViewport` _output_get 0)
    (`GameplayStatics.SetGamePaused` true)))

(event `Key|U`
  (params (Key :type "Key Structure"))
  (:`Pressed`
    (`/Game/UEGameCode/Core/Blueprints/BP_HUD_Base_LEGACY.Toggle_UpgradesPanel` (`self.As BP HUD Base`))))

(event `EnhancedInput|/Game/UEGameCode/Core/Input/Actions/IA_Restart`
  (params (ActionValue :type Boolean) (ElapsedSeconds :type "Float (double-precision)") (TriggeredSeconds :type "Float (double-precision)") (InputAction :type "InputAction Object Reference" :default "/Game/UEGameCode/Core/Input/Actions/IA_Restart.IA_Restart"))
  (:`Triggered`
    (bind _asbp_dark_rage_character_legacy (cast `/Game/UEGameCode/Core/Blueprints/BP_DarkRageCharacter_LEGACY` (`self.K2_GetPawn`)))
    (`/Game/UEGameCode/Core/Blueprints/BP_DarkRageCharacter_LEGACY.CallRestartPlayer` _asbp_dark_rage_character_legacy)))

(fn `UserConstructionScript`)