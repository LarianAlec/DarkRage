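; BP_DRPlayerController is the DarkRage player controller, adding debug keys for restarting and pausing during testing.
; The first debug numpad key triggers a hot reload, which destroys actors reported by the player character, unpossesses it and restarts the player at the DRPlayerStart spot without reloading the map.
; The second key toggles game pause through a FlipFlop.
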(event Custom|HotReload
  (CallFunction|HOTRELOADLEVELDEBUG))

(event EventBeginPlay
  (|CallParentFunction)
  (Utilities|FlowControl|Sequence))

(event Input|KeyboardEvents|DebugKeyNumPadOne
  (params (Key :type Key%20Structure) (ActionValue :type Input%20Action%20Value%20Structure))
  (:Pressed
    (CallFunction|HotReload)))

(event Input|KeyboardEvents|DebugKeyNumPadTwo
  (params (Key :type Key%20Structure) (ActionValue :type Input%20Action%20Value%20Structure))
  (:Pressed
    (Utilities|FlowControl|FlipFlop
      (:A
        (Game|SetGamePaused true))
      (:B
        (Game|SetGamePaused false)))))

(fn ConstructionScript)

(fn HOTRELOADLEVELDEBUG
  (bind _returnvalue (Game|GetGameMode))
  (bind _returnvalue_2 (Game|GetPlayerController 0))
  (bind _asbp_dark_rage_character_actual (Utilities|Casting|CastToBP_DarkRageCharacter_Actual (Game|GetPlayerCharacter 0)))
  (bind _actorstodestroy (Default|GetAllActorstoDestroy _asbp_dark_rage_character_actual))
  (bind _output_get (Variables|Default|SetActorsToDestroy _actorstodestroy))
  (for _array_element _output_get
    (Utilities|IsValid _array_element
      (:Is%20Valid
        (Actor|DestroyActor _array_element))))
  (Pawn|UnPossess _returnvalue_2)
  (Class|GameModeBase|RestartPlayeratPlayerStart _returnvalue _returnvalue_2 (Class|GameModeBase|FindPlayerStart _returnvalue _returnvalue_2 "DRPlayerStart")))