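; BP_DarkRageGameMode_LEGACY is a legacy game mode that shows the death menu when the player dies.
; On BeginPlay it binds PlayerDied to the OnPlayerDied dispatcher, then caches the first player's pawn and HUD as their legacy Dark Rage classes.
; When the dispatcher fires, PlayerDied calls ShowDeathMenu on the cached HUD.
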(event `self.ReceiveBeginPlay`
  (add `self.OnPlayerDied` (delegate `PlayerDied`))
  (bind _asbp_dark_rage_character (cast `/Game/UEGameCode/Core/Blueprints/BP_DarkRageCharacter_LEGACY` (`Controller.K2_GetPawn` (`GameplayStatics.GetPlayerController` 0))))
  (set `self.PlayersPawn` _asbp_dark_rage_character)
  (bind _asbp_hud_base (cast `/Game/UEGameCode/Core/Blueprints/BP_HUD_Base_LEGACY` (`PlayerController.GetHUD` (`GameplayStatics.GetPlayerController` 0))))
  (set `self.PlayersHUD` _asbp_hud_base))

(event `PlayerDied`
  (`/Game/UEGameCode/Core/Blueprints/BP_HUD_Base_LEGACY.ShowDeathMenu` (`self.PlayersHUD`)))

(fn `UserConstructionScript`)