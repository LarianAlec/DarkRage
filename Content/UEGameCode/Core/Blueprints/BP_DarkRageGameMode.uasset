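; BP_DarkRageGameMode is a game mode that shows the death menu when the player dies.
; On BeginPlay it binds to its OnPlayerDied event, then caches the first player's pawn as BP_DarkRageCharacter and its HUD as BP_HUD_Base.
; When the event fires, it calls ShowDeathMenu on the cached HUD, which is only set if both casts succeed.
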(event `self.ReceiveBeginPlay`
  (add `self.OnPlayerDied` (delegate `PlayerDied`))
  (bind _asbp_dark_rage_character (cast `/Game/UEGameCode/Core/Blueprints/BP_DarkRageCharacter` (`Controller.K2_GetPawn` (`GameplayStatics.GetPlayerController` 0))))
  (set `self.PlayersPawn` _asbp_dark_rage_character)
  (bind _asbp_hud_base (cast `/Game/UEGameCode/Core/Blueprints/BP_HUD_Base` (`PlayerController.GetHUD` (`GameplayStatics.GetPlayerController` 0))))
  (set `self.PlayersHUD` _asbp_hud_base))

(event `PlayerDied` :!signature `self.OnPlayerDied`
  (params (Character :type "/Game/UEGameCode/Core/Blueprints/BP_DarkRageCharacter Object Reference"))
  (`/Game/UEGameCode/Core/Blueprints/BP_HUD_Base.ShowDeathMenu` (`self.PlayersHUD`)))

(fn `UserConstructionScript`)