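; BP_DarkRagePlayerController is a player controller that sets up Enhanced Input and opens the pause menu.
; On BeginPlay it casts player controller 0 to itself and adds the IMC_FirstPersonPlayer mapping context.
; IA_CallMenu creates a new WBP_PauseMenu, adds it to the viewport and pauses the game.
; The pause toggle branch is disconnected, so this controller only pauses and never unpauses.
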(event `self.ReceiveBeginPlay`
  ;[1 0.2059 0.2656 1 50] ENHANCED INPUT SYSTEM Add Input Mapping
  (bind _asbp_dark_rage_player_controller (cast `/Game/UEGameCode/Core/Blueprints/BP_DarkRagePlayerController` (`GameplayStatics.GetPlayerController` 0)))
  (bind _returnvalue (pcsubsystem `EnhancedInputLocalPlayerSubsystem` _asbp_dark_rage_player_controller))
  (`/Engine/EditorBlueprintResources/StandardMacros.IsValid` _returnvalue
    (:`Is Valid`
      (`EnhancedInputSubsystemInterface.AddMappingContext` _returnvalue "/Game/UEGameCode/Core/Input/IMC_FirstPersonPlayer.IMC_FirstPersonPlayer" 0 (struct)))))

(event `EnhancedInput|/Game/UEGameCode/Core/Input/Actions/IA_CallMenu`
  (params (ActionValue :type Boolean) (ElapsedSeconds :type "Float (double-precision)") (TriggeredSeconds :type "Float (double-precision)") (InputAction :type "InputAction Object Reference" :default "/Game/UEGameCode/Core/Input/Actions/IA_CallMenu.IA_CallMenu"))
  (:`Triggered`
    (set `self.IsGamePaused` true)
    (bind _returnvalue (`|CreateWidget` "/Game/UEGameCode/UI/WBP_PauseMenu.WBP_PauseMenu_C" (`GameplayStatics.GetPlayerController` 0)))
    (bind _output_get (set `self.PauseMenuWidget` _returnvalue))
    (`UserWidget.AddToViewport` _output_get 0)
    (`GameplayStatics.SetGamePaused` true)))

(fn `UserConstructionScript`)