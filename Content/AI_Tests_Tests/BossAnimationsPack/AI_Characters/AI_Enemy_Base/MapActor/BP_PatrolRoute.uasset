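; BP_PatrolRoute is a map actor that defines a patrol path for AI enemies with a PatrolRoute spline.
; GetSplaneSpotsAsWorldPosition returns the world location of the spline point at the current PatrolIndex.
; IncreamentPatrolRoute steps the index by Deraction and flips that direction at the first and last points, giving a back-and-forth ping-pong route.
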(event `IncreamentPatrolRoute`
  (bind _output_get (set `self.PatrolIndex` (+ (`self.PatrolIndex`) (`self.Deraction`))))
  (if (== _output_get (- (`SplineComponent.GetNumberOfSplinePoints` (`self.PatrolRoute`)) 1))
    (set `self.Deraction` -1)
    (elif (== (`self.PatrolIndex`) 0)
      (set `self.Deraction` 1))))

(fn `Get Splane Spots as World Position`
  (returns (Location :type "Vector Structure"))
  (return (`SplineComponent.GetLocationAtSplinePoint` (`self.PatrolRoute`) (`self.PatrolIndex`) "World")))

(fn `UserConstructionScript`)