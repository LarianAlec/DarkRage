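; BP_EnemyArrow is an enemy bow projectile that damages the actor it hits.
; On box overlap, ignoring itself and actors tagged "Arrow", it stops movement, zeroes gravity and attaches to the hit actor.
; It sends damage through a TakeDamage message with a damage-info struct, plays a hit sound for the player character class, then destroys itself immediately.
; A second sequence branch disables box collision if the box is still valid.
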(event `self.Box.OnComponentBeginOverlap`
  (params (OverlappedComponent :type "PrimitiveComponent Object Reference") (OtherActor :type "Actor Object Reference") (OtherComp :type "PrimitiveComponent Object Reference") (OtherBodyIndex :type Integer) (bFromSweep :type Boolean) (SweepResult :type "HitResult Structure (by ref)"))
  (bind _projectilemovement (`self.ProjectileMovement`))
  (bind _box (`self.Box`))
  (bind _hittedactor (`self.HittedActor`))
  (if (and (!= OtherActor self) (not (`self.ActorHasTag` OtherActor "Arrow")))
    (set `self.HittedActor` OtherActor)
    (`MovementComponent.StopMovementImmediately` _projectilemovement)
    (set `ProjectileMovementComponent.ProjectileGravityScale` 0.0 _projectilemovement)
    (`self.K2_AttachToActor` OtherActor "None" "KeepWorld" "KeepWorld" "KeepWorld")
    (`|ExecutionSequence`
      (:`then_0`
        (message `/Game/DarkRage/Core/Blueprints/DamageSystem/BPI_DRDamageSystem.TakeDamage` (`self.HittedActor`) (make `/Game/DarkRage/Core/Blueprints/DamageSystem/S_DRDamageInfo` (`self.ArrowDamage`) "NewEnumerator2" "NewEnumerator1") null)
        (cast `/Game/DarkRage/Core/Characters/DarkRageCharacter/BP_DarkRageCharacter_Actual` _hittedactor
          (:`then`
            (`GameplayStatics.SpawnSoundAtLocation` "/Game/DarkRage/Core/SFX/Bow/A_BowHit_3_Cue.A_BowHit_3_Cue" (`self.K2_GetActorLocation` _hittedactor) (struct) 1.0 1.0 0.0 "/Game/DarkRage/Core/SFX/EnemyMelee/ATT_Melee.ATT_Melee" null))
          (:`CastFailed`
            _))
        (`self.K2_DestroyActor`))
      (:`then_1`
        (`/Engine/EditorBlueprintResources/StandardMacros.IsValid` _box
          (:`Is Valid`
            (`PrimitiveComponent.SetCollisionEnabled` _box "NoCollision")))))))

(fn `UserConstructionScript`)