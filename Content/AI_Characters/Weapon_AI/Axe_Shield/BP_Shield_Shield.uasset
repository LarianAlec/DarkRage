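; Shield Blueprint for the AI axe-and-shield weapon set, reacting to point-damage hits.
; On BeginPlay it runs parent logic, then binds point damage to play a light wood bullet-impact sound and make noise at the hit location.
; Tick polls the Dead flag and destroys the AbsorbArea component once it is set, if that component is still valid.
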(event `self.ReceiveTick`
  (params (DeltaSeconds :type "Float (single-precision)"))
  (if (`self.Dead`)
    (bind _absorbarea (`self.AbsorbArea`)
      (:`then`
        (`ActorComponent.K2_DestroyComponent` _absorbarea))
      (:`else`))))

(event `self.ReceiveBeginPlay`
  (`parent.ReceiveBeginPlay`)
  (add `self.OnTakePointDamage` (delegate `OnTakePointDamage_Event`)))

(event `OnTakePointDamage_Event` :!signature `self.OnTakePointDamage`
  (params (DamagedActor :type "Actor Object Reference") (Damage :type "Float (single-precision)") (InstigatedBy :type "Controller Object Reference") (HitLocation :type "Vector Structure") (FHitComponent :type "PrimitiveComponent Object Reference") (BoneName :type Name) (ShotFromDirection :type "Vector Structure") (DamageType :type "DamageType Object Reference") (DamageCauser :type "Actor Object Reference"))
  (`GameplayStatics.PlaySoundAtLocation` "/Game/Sound/Sound/ProSoundCollection/GunsWeapons/Bullets/Wavs/bullet_impact_wood_light_01_Cue.bullet_impact_wood_light_01_Cue" HitLocation (struct) 1.0 1.0 0.0 null null null null)
  (`self.MakeNoise` 1.0 null HitLocation))

(fn `UserConstructionScript`
  (`parent.UserConstructionScript`))