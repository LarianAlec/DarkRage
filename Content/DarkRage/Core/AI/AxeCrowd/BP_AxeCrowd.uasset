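; Axe-wielding crowd enemy AI character that extends a parent class with melee attacks, weapon equip and unequip, per-state walk speeds and ideal combat ranges.
; Attacks play a random montage, whose trace notify sphere-traces forward and damages non-AI actors with hit or whoosh sounds.
; BPC DR damage system holds health and is uninterruptable during attacks.
; Equip and unequip montage notifies spawn, socket-attach and destroy the axe.
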(event `self.ReceiveBeginPlay`
  (`parent.ReceiveBeginPlay`)
  (set `/Game/DarkRage/Core/Blueprints/DamageSystem/BPC_DRDamageSystem.Health` (`self.Health`) (`self.BPC_DRDamageSystem`)))

(event `/Game/DarkRage/Core/AI/Character/Interfaces/BPI_AICharacter.Attack`
  (params (AttackTarget :type "Actor Object Reference"))
  (bind _returnvalue (`self.K2_GetActorLocation`))
  (bind _bpc_drdamagesystem (`self.BPC_DRDamageSystem`))
  ;[1 0 0] Attack Event
  (`parent.Attack` AttackTarget)
  (bind _notifyname (`|PlayMontage` (`self.Mesh`) (`KismetArrayLibrary.Array_Random` (`self.AttackMontages`)))
    (:`then`
      (`self.OnAttackStarted`)
      (set `/Game/DarkRage/Core/Blueprints/DamageSystem/BPC_DRDamageSystem.IsInterruptable` false _bpc_drdamagesystem))
    (:`OnCompleted`
      (`/Game/DarkRage/Core/AI/Character/Interfaces/BPI_AICharacter.AttackEnd` AttackTarget :!label _label)
      (set `/Game/DarkRage/Core/Blueprints/DamageSystem/BPC_DRDamageSystem.IsInterruptable` true _bpc_drdamagesystem))
    (:`OnInterrupted`
      (goto _label))
    (:`OnNotifyBegin`
      (switch `name` _notifyname
        (:`AttackTrace`
          (bind (_outhit _returnvalue_2) (`KismetSystemLibrary.SphereTraceSingleForObjects` _returnvalue (+ _returnvalue (* (`self.GetActorForwardVector`) (`self.AttackRange`))) 30.0 (`|MakeArray` "ObjectTypeQuery3" :!type "EObjectTypeQuery Enum")))
          (if _returnvalue_2
            (bind (_bblockinghit _binitialoverlap _time _distance _location _impactpoint _normal _impactnormal _physmat _hitactor) (`GameplayStatics.BreakHitResult` _outhit))
            (if (not (`KismetSystemLibrary.DoesImplementInterface` _hitactor "/Game/DarkRage/Core/AI/Character/Interfaces/BPI_AICharacter.BPI_AICharacter_C"))
              (message `/Game/DarkRage/Core/Blueprints/DamageSystem/BPI_DRDamageSystem.TakeDamage` _hitactor (make `/Game/DarkRage/Core/Blueprints/DamageSystem/S_DRDamageInfo` (`self.DamageAmount`) "NewEnumerator1" "NewEnumerator1") null)
              (`GameplayStatics.SpawnSoundAtLocation` "/Game/DarkRage/Core/SFX/EnemyMelee/A_SwordHit_Cue.A_SwordHit_Cue" _impactpoint (struct) 1.0 1.0 0.0 "/Game/DarkRage/Core/SFX/EnemyMelee/ATT_Melee.ATT_Melee" null))
            (else
              (`GameplayStatics.SpawnSoundAtLocation` "/Game/DarkRage/Core/SFX/EnemyMelee/A_Woosh_Cue.A_Woosh_Cue" (`self.K2_GetActorLocation`) (struct) 1.0 1.0 0.0 "/Game/DarkRage/Core/SFX/EnemyMelee/ATT_Melee.ATT_Melee" null))))))))

(event `/Game/DarkRage/Core/AI/Character/Interfaces/BPI_AICharacter.EquipWeapon`
  ;[1 0.3551 0] Equip Weapon
  (if (not (`self.IsArmed`))
    (bind _notifyname (`|PlayMontage` (`self.Mesh`) "/Game/DarkRage/Core/AI/AxeCrowd/Animations/Shield/AM_AxeCrowd_Equip.AM_AxeCrowd_Equip")
      (:`then`
        (`self.OnEquipWeaponStart`))
      (:`OnCompleted`
        (`self.OnEquipWeaponEnd` :!label _label_2))
      (:`OnNotifyBegin`
        (switch `name` _notifyname
          (:`AttachWeaponToSocket`
            (bind _returnvalue (`|SpawnActorFromClass` "/Game/DarkRage/Core/Weapons/Axe1H/BP_Axe1H.BP_Axe1H_C" (`self.GetTransform`) "Undefined" "MultiplyWithRoot" null null))
            (bind _output_get (set `self.WeaponActor` _returnvalue))
            (`self.K2_AttachToComponent` _output_get (`self.Mesh`) "RHandAxeSocket" "SnapToTarget" "SnapToTarget" "SnapToTarget" true)
            (set `self.IsArmed` true))
          (:`EndOfEquip`
            (goto _label_2)))))))

(event `/Game/DarkRage/Core/AI/Character/Interfaces/BPI_AICharacter.UnequipWeapon`
  ;[1 0.3551 0] Unequip weapon
  (if (`self.IsArmed`)
    (bind _notifyname (`|PlayMontage` (`self.Mesh`) "/Game/DarkRage/Core/AI/AxeCrowd/Animations/Shield/AM_AxeCrowd_Unequip.AM_AxeCrowd_Unequip")
      (:`then`
        (`self.OnUnequipWeaponStart`))
      (:`OnCompleted`
        (`self.OnUnequipWeaponEnd` :!label _label_3)
        (set `self.IsArmed` false))
      (:`OnInterrupted`
        (goto _label_3))
      (:`OnNotifyBegin`
        (switch `name` _notifyname
          (:`DetachWeaponFromSocket`
            (`self.K2_DestroyActor` (`self.WeaponActor`))))))))

(fn `GetIdealRange`
  (returns (AttackRadius :type "Float (double-precision)") (DefendRadius :type "Float (double-precision)"))
  (return (`self.AttackRadius`) (`self.StrafeRadius`)))

(fn `SetMovementSpeed`
  (params (NewSpeed :type "/Game/DarkRage/Core/AI/Character/Enums/E_MovementAISpeed Enum" :default "NewEnumerator0"))
  (returns (CurrentSpeed :type "Float (double-precision)"))
  (bind _output_get (set `CharacterMovementComponent.MaxWalkSpeed` (select `/Game/DarkRage/Core/AI/Character/Enums/E_MovementAISpeed` NewSpeed :`NewEnumerator1` (`self.WalkingSpeed`) :`NewEnumerator4` (`self.StrafingSpeed`) :`NewEnumerator2` (`self.JoggingSpeed`) :`NewEnumerator3` (`self.SprintingSpeed`) :!type "Float (single-precision)") (`self.CharacterMovement`)))
  (return _output_get))

(fn `UserConstructionScript`
  (`parent.UserConstructionScript`))